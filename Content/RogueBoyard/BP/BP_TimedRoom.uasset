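; BP_TimedRoom is a room Blueprint for a timed challenge room in RogueBoyard.
; On BeginPlay it caches the player's HUD_Rogue, printing an error if the cast fails.
; When the room is entered, it reveals the player 1 MJ image on the timed-room title card, shows that card and starts the HUD chrono.
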(event EventRoomEnter
  (bind _hud (Variables|Default|GetHUD))
  (Variables|/Script/UMG.Widget|SetVisibility (Variables|/Game/RogueBoyard/UMG/TitleCards/W_TimedRoom_TitleCard.W_TimedRoom_TitleCard_C|GetP1_MJ_Img (Variables|/Game/RogueBoyard/Core/HUD_Rogue.HUD_Rogue_C|GetTimedRoomTC _hud)) "Visible")
  (Default|CEShowTitleCard _hud (Variables|/Game/RogueBoyard/Core/HUD_Rogue.HUD_Rogue_C|GetTimedRoomTC _hud))
  (Default|CEStartChrono (Variables|Default|GetHUD)))

(event EventBeginPlay
  (bind _ashud_rogue (Utilities|Casting|CastToHUD_Rogue (HUD|GetHUD (Game|GetPlayerController 0)))
    (:then
      (Variables|Default|SetHUD _ashud_rogue))
    (:CastFailed
      (Development|PrintString "cast failed"))))

(fn ConstructionScript)