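; BP_CameraView is a menu station actor that hosts a menu widget and serves as a camera view target for moving between menus.
; On BeginPlay it casts its widget to MainMenuParentClass, prints its name as debug and binds to the menu transition event.
; That event's index selects an entry in LinkedMenus; the actor then swaps collision to that menu and eases the player's view over to it.
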(event Custom|CE_TransitionTo
  (params (Menu :type BP%20Camera%20View%20Object%20Reference))
  (Collision|SetActorEnableCollision false)
  (Collision|SetActorEnableCollision Menu true)
  (Game|Player|SetViewTargetwithBlend (Game|GetPlayerController 0) Menu 1.0 "VTBlend_EaseInOut" 2.0 false))

(event Custom|OnTransitionBetweenMenus
  (params (MenuIndex :type Integer))
  (if (Utilities|Array|IsValidIndex (Variables|Default|GetLinkedMenus) MenuIndex)
    (CallFunction|CETransitionto (Utilities|Array|Get(acopy) (Variables|Default|GetLinkedMenus) MenuIndex))))

(event EventBeginPlay
  (bind _asmain_menu_parent_class (Utilities|Casting|CastToMainMenuParentClass (UserInterface|GetUserWidgetObject (Variables|Default|GetWidgetComponent))))
  (Development|PrintString (Utilities|GetDisplayName _asmain_menu_parent_class) true true "(R=1.000000,G=0.000000,B=0.000000,A=1.000000)" 1e+01)
  (EventDispatchers|AssignOnMenuTransition _asmain_menu_parent_class (delegate Custom|OnTransitionBetweenMenus)))

(fn ConstructionScript)