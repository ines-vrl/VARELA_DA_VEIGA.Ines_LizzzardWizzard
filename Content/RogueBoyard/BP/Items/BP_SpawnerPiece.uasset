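; BP_SpawnerPiece is a spawner actor that periodically drops coins at random points within a zone.
; Tick accumulates delta time and, once it exceeds TimeBetweenSpawnPiece, resets the timer and calls the spawn dispatch.
; The spawn event creates a CoinToSpawn actor at a random point in the ZoneSpawnPiece box and gives it a limited lifespan.
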(event Custom|ED_SpawnPiece
  (bind _zonespawnpiece (Variables|Default|GetZoneSpawnPiece))
  (bind _returnvalue (Game|SpawnActorfromClass (Variables|SpawnerPiece|GetCoinToSpawn) (Math|Transform|MakeTransform (Math|Random|RandomPointinBoundingBox (Transformation|GetWorldLocation _zonespawnpiece) (Components|Box|GetScaledBoxExtent _zonespawnpiece)) "0, 0, 0" "1.000000,1.000000,1.000000") "Undefined" "MultiplyWithRoot" 0 0))
  (Actor|SetLifeSpan _returnvalue (Variables|SpawnerPiece|GetLifespanCoin)))

(event EventTick
  (params (DeltaSeconds :type Float%20%28single-precision%29))
  (CallFunction|Tick DeltaSeconds))

(fn ConstructionScript)

(fn Tick
  (params (DeltaTime :type Float%20%28double-precision%29))
  (bind _output_get (Variables|Default|SetTimer (+ DeltaTime (Variables|Default|GetTimer))))
  (if (< (Variables|SpawnerPiece|GetTimeBetweenSpawnPiece) _output_get)
    (Variables|Default|SetTimer 0.0)
    (CallFunction|EDSpawnPiece)))