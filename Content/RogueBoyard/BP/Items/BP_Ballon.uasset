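; Physics-style ball that bounces off walls and knocks rogue characters away in RogueBoyard.
; Tick calls MovingOnSin while movement is enabled; sphere overlaps drive the collision responses.
; Wall_P hits briefly freeze movement for a speed-scaled time, then apply an impulse along the reflected velocity.
; Fast hits push non-dashing RogueCharacters through their PushableComponent, then send the ball a zero impulse.
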(event OnComponentBeginOverlap(Sphere1)
  (params (OverlappedComponent :type Primitive%20Component%20Object%20Reference) (OtherActor :type Actor%20Object%20Reference) (OtherComp :type Primitive%20Component%20Object%20Reference) (OtherBodyIndex :type Integer) (bFromSweep :type Boolean) (SweepResult :type Hit%20Result%20Structure%20%28by%20ref%29))
  (bind _returnvalue (Actor|GetComponentbyClass OtherActor "/Script/RogueBoyard.PushableComponent"))
  (Utilities|Casting|CastToWall_P OtherActor
    (:then
      (Variables|Default|SetCanMove false)
      (Utilities|FlowControl|Delay (Math|Float|Lerp (Variables|Default|GetTimeFreezeMin) (Variables|Default|GetTimeFreezeMax) (/ (Math|Vector|VectorLength (Variables|Default|GetVelocity)) (Variables|Default|GetMaxSpeed))))
      (Variables|Default|SetCanMove true)
      (Class|Ballon|AddImpulse (Math|Vector|GetReflectionVector (Variables|Default|GetVelocity) (.impactnormal SweepResult)) true))
    (:CastFailed
      (Utilities|IsValid _returnvalue
        (:Is%20Valid
          (if (>= (Math|Vector|VectorLength (Variables|Default|GetVelocity)) (* (Variables|Default|GetMaxSpeed) 0.4))
            (bind _asrogue_character (Utilities|Casting|CastToRogueCharacter OtherActor))
            (Development|PrintString (Utilities|String|EnumtoString (Variables|/Script/RogueBoyard.RogueCharacterStateMachine|GetCurrentStateID (Variables|/Script/RogueBoyard.RogueCharacter|GetStateMachine _asrogue_character))))
            (if (not (Utilities|Enum|Equal(Enum) (Variables|/Script/RogueBoyard.RogueCharacterStateMachine|GetCurrentStateID (Variables|/Script/RogueBoyard.RogueCharacter|GetStateMachine _asrogue_character)) "Dash"))
              (Class|PushableComponent|Push _returnvalue (* (Variables|Default|GetVelocity) (Variables|Default|GetEjectionResistance)) 1.0)
              (Class|Ballon|AddImpulse "0, 0, 0" true))))))))

(event EventBeginPlay
  (Variables|Default|SetStartScale (Variables|/Script/Engine.SceneComponent|GetRelativeScale3D (Variables|Default|GetSphere1)))
  (Development|PrintString (Utilities|String|ToString(Vector) (Variables|Default|GetStartScale))))

(event Collision|EventActorBeginOverlap
  (params (OtherActor :type Actor%20Object%20Reference)))

(event EventTick
  (params (DeltaSeconds :type Float%20%28single-precision%29))
  (if (Variables|Default|GetCanMove)
    (Class|Ballon|MovingonSin)))

(fn ConstructionScript)