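; Lobby room Blueprint that drives the HUD timers for a vote and for the room itself.
; BeginPlay caches the first player's HUD_Rogue, and BeginRoom hides the title card and starts the room timer.
; Tick watches IsVoteActive, using latch booleans to start or end the vote timer once per change and updating the remaining time while voting runs.
; EndRoom ends both timers.
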(event EventBeginRoom
  (Default|CEHideTitleCardSimon (Variables|Default|GetHUD))
  (Default|CEStartRoomTimer (Variables|Default|GetHUD) (Variables|Default|GetMaxRoomTime)))

(event EventBeginPlay
  (bind _ashud_rogue (Utilities|Casting|CastToHUD_Rogue (HUD|GetHUD (Game|GetPlayerController 0))))
  (Variables|Default|SetHUD _ashud_rogue))

(event EventEndRoom
  (Default|CEEndRoomTimer (Variables|Default|GetHUD))
  (Default|CEEndVoteTimer (Variables|Default|GetHUD)))

(event EventTick
  (params (DeltaSeconds :type Float%20%28single-precision%29))
  (bind _hud (Variables|Default|GetHUD))
  (if (Variables|Default|GetbIsVoteActive)
    (if (not (Variables|Default|GetStartTimer))
      (Default|CEStartVoteTimer _hud)
      (Variables|Default|SetStartTimer true)
      (Variables|Default|SetEndTimer false)
      (else
        (Default|CESetVoteTimerValue _hud (- (Variables|Default|GetVoteTimer) (Variables|Default|GetElapsedTime)))))
    (elif (not (Variables|Default|GetEndTimer))
      (Default|CEEndVoteTimer (Variables|Default|GetHUD))
      (Variables|Default|SetEndTimer true)
      (Variables|Default|SetStartTimer false))))

(fn ConstructionScript)