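; Millstone trap: four cylinders roll around a central rotating pivot, and characters that begin overlapping its box take damage.
; At BeginPlay it caches each cylinder's Y offset and the pivot's Z as a radius, then requests per-cylinder spin speeds from CalculateSpeedRotation, whose distance-to-radius scaling nodes are marked unused.
; Tick yaws the pivot and pitches the cylinders by fixed per-frame amounts unscaled by delta time, with ClockwiseRotation setting the direction.
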(event OnComponentBeginOverlap(Box)
  (params (OverlappedComponent :type Primitive%20Component%20Object%20Reference) (OtherActor :type Actor%20Object%20Reference) (OtherComp :type Primitive%20Component%20Object%20Reference) (OtherBodyIndex :type Integer) (bFromSweep :type Boolean) (SweepResult :type Hit%20Result%20Structure%20%28by%20ref%29))
  (bind _asbp_character (Utilities|Casting|CastToBP_Character OtherActor))
  (Class|RogueCharacter|TakeDamage _asbp_character (Variables|Default|GetDamage)))

(event EventTick
  (params (DeltaSeconds :type Float%20%28single-precision%29))
  (if (Variables|Trap|Millstone|GetClockwiseRotation)
    (Transformation|AddRelativeRotation (Variables|Default|GetPivotRotation) (Math|Rotator|MakeRotator 0.0 0.0 (Variables|Trap|Millstone|GetSpeedRotation)) false false)
    (Transformation|AddLocalRotation (Variables|Default|GetMillestoneCylinderInt) (Math|Rotator|MakeRotator 0.0 (Variables|Default|GetSCylinderInt) 0.0) false false)
    (Transformation|AddLocalRotation (Variables|Default|GetMillestoneCylinder1) (Math|Rotator|MakeRotator 0.0 (Variables|Default|GetSCylinder1) 0.0) false false)
    (Transformation|AddLocalRotation (Variables|Default|GetMillestoneCylinder2) (Math|Rotator|MakeRotator 0.0 (Variables|Default|GetSCylinder2) 0.0) false false)
    (Transformation|AddLocalRotation (Variables|Default|GetMillestoneCylinderExt) (Math|Rotator|MakeRotator 0.0 (Variables|Default|GetSCylinderExt) 0.0) false false)
    (else
      (Transformation|AddRelativeRotation (Variables|Default|GetPivotRotation) (Math|Rotator|MakeRotator 0.0 0.0 (* (Variables|Trap|Millstone|GetSpeedRotation) -1.0)) false false)
      (Transformation|AddLocalRotation (Variables|Default|GetMillestoneCylinderInt) (Math|Rotator|MakeRotator 0.0 (* (Variables|Default|GetSCylinderInt) -1.0) 0.0) false false)
      (Transformation|AddLocalRotation (Variables|Default|GetMillestoneCylinder1) (Math|Rotator|MakeRotator 0.0 (* (Variables|Default|GetSCylinder1) -1.0) 0.0) false false)
      (Transformation|AddLocalRotation (Variables|Default|GetMillestoneCylinder2) (Math|Rotator|MakeRotator 0.0 (* (Variables|Default|GetSCylinder2) -1.0) 0.0) false false)
      (Transformation|AddLocalRotation (Variables|Default|GetMillestoneCylinderExt) (Math|Rotator|MakeRotator 0.0 (* (Variables|Default|GetSCylinderExt) -1.0) 0.0) false false))))

(event EventBeginPlay
  (Variables|Default|SetDCylinder1 (.y (Variables|/Script/Engine.SceneComponent|GetRelativeLocation (Variables|Default|GetMillestoneCylinder1))))
  (Variables|Default|SetDCylinder2 (.y (Variables|/Script/Engine.SceneComponent|GetRelativeLocation (Variables|Default|GetMillestoneCylinder2))))
  (Variables|Default|SetDCylinderExt (.y (Variables|/Script/Engine.SceneComponent|GetRelativeLocation (Variables|Default|GetMillestoneCylinderExt))))
  (Variables|Default|SetDCylinderInt (.y (Variables|/Script/Engine.SceneComponent|GetRelativeLocation (Variables|Default|GetMillestoneCylinderInt))))
  (Variables|Default|SetRCylinder (.z (Variables|/Script/Engine.SceneComponent|GetRelativeLocation (Variables|Default|GetPivotRotation))))
  (Variables|Default|SetSCylinderInt (Utilities|CalculateSpeedRotation (Variables|Default|GetDCylinderInt)))
  (Variables|Default|SetSCylinder1 (Utilities|CalculateSpeedRotation (Variables|Default|GetDCylinder1)))
  (Variables|Default|SetSCylinder2 (Utilities|CalculateSpeedRotation (Variables|Default|GetDCylinder2)))
  (Variables|Default|SetSCylinderExt (Utilities|CalculateSpeedRotation (Variables|Default|GetDCylinderExt))))

(fn ConstructionScript)