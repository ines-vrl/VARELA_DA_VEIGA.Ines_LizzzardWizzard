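; Millstone trap that turns around a central pivot once Init is called and damages any BP_Character entering its box.
; Tick yaws the pivot by SpeedRotation in either direction, scaled by delta time only when clockwise.
; BeginPlay derives three cylinder roll speeds from their offsets via CalculateSpeedRotation, whose speed-ratio math is unconnected.
; SetRotation receives those speeds but multiplies pitch by zero, so the cylinders get no spin.
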(event OnComponentBeginOverlap(Box)
  (params (OverlappedComponent :type Primitive%20Component%20Object%20Reference) (OtherActor :type Actor%20Object%20Reference) (OtherComp :type Primitive%20Component%20Object%20Reference) (OtherBodyIndex :type Integer) (bFromSweep :type Boolean) (SweepResult :type Hit%20Result%20Structure%20%28by%20ref%29))
  (bind _asbp_character (Utilities|Casting|CastToBP_Character OtherActor))
  (Class|RogueCharacter|TakeDamage _asbp_character (Variables|Default|GetDamage)))

(event EventTick
  (params (DeltaSeconds :type Float%20%28single-precision%29))
  (Variables|Default|SetDelta%20Seconds DeltaSeconds)
  (if (Variables|Default|GetIsInit)
    (if (Variables|Trap|Millstone|GetClockwiseRotation)
      (Transformation|AddRelativeRotation (Variables|Default|GetPivotRotation) (Math|Rotator|MakeRotator 0.0 0.0 (* (Variables|Trap|Millstone|GetSpeedRotation) (Variables|Default|GetDelta%20Seconds))) false false)
      (CallFunction|SetRotation (Variables|Default|GetMillestoneCylinderInt) (Variables|Default|GetSCylinderInt))
      (CallFunction|SetRotation (Variables|Default|GetMillestoneCylinder1) (Variables|Default|GetSCylinder1))
      (CallFunction|SetRotation (Variables|Default|GetMillestoneCylinderExt) (Variables|Default|GetSCylinderExt))
      (else
        (Transformation|AddRelativeRotation (Variables|Default|GetPivotRotation) (Math|Rotator|MakeRotator 0.0 0.0 (* (Variables|Trap|Millstone|GetSpeedRotation) -1.0)) false false)
        (CallFunction|SetRotation (Variables|Default|GetMillestoneCylinderInt) (* (Variables|Default|GetSCylinderInt) -1.0))
        (CallFunction|SetRotation (Variables|Default|GetMillestoneCylinder1) (* (Variables|Default|GetSCylinder1) -1.0))
        (CallFunction|SetRotation (Variables|Default|GetMillestoneCylinderExt) (* (Variables|Default|GetSCylinderExt) -1.0))))))

(event EventBeginPlay
  (Variables|Default|SetDCylinder1 (.y (Variables|/Script/Engine.SceneComponent|GetRelativeLocation (Variables|Default|GetMillestoneCylinder1))))
  (Variables|Default|SetDCylinderExt (.y (Variables|/Script/Engine.SceneComponent|GetRelativeLocation (Variables|Default|GetMillestoneCylinderExt))))
  (Variables|Default|SetDCylinderInt (.y (Variables|/Script/Engine.SceneComponent|GetRelativeLocation (Variables|Default|GetMillestoneCylinderInt))))
  (Variables|Default|SetRCylinder (.z (Variables|/Script/Engine.SceneComponent|GetRelativeLocation (Variables|Default|GetPivotRotation))))
  (Variables|Default|SetSCylinderInt (Utilities|CalculateSpeedRotation (Variables|Default|GetDCylinderInt)))
  (Variables|Default|SetSCylinder1 (Utilities|CalculateSpeedRotation (Variables|Default|GetDCylinder1)))
  (Variables|Default|SetSCylinderExt (Utilities|CalculateSpeedRotation (Variables|Default|GetDCylinderExt))))

(event EventInit
  (Variables|Default|SetIsInit true))

(fn ConstructionScript)

(fn SetRotation
  (params (self2 :type Scene%20Component%20Object%20Reference) (A :type Float%20%28double-precision%29))
  (Transformation|AddLocalRotation self2 (Math|Rotator|MakeRotator 0.0 (* A 0.0) 0.0) false false))