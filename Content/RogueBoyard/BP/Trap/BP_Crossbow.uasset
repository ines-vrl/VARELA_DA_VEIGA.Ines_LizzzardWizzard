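; BP_Crossbow is a trap that fires charged BP_Arrow projectiles.
; Started or the O key begins charging if a shot is available, and Tick raises shot strength until it reaches MaxSpeed.
; Stopped or P spawns an arrow at DirectionalArrow with that strength and configurable physics and damage, then resets and re-enables charging after a delay.
; Release does not check CanShoot or Charge, so it always spawns an arrow.
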(event EventBeginPlay
  (bind _returnvalue (Actor|GetActorOfClass "/Game/RogueBoyard/BP/Trap/BP_Arrow.BP_Arrow_C"))
  (Variables|Default|SetCrossbowArrow _returnvalue))

(event EventReleaseShot
  ;[0.1385 0.1385 0.1385] Release shoot
  (Game|SpawnActorfromClass "/Game/RogueBoyard/BP/Trap/BP_Arrow.BP_Arrow_C" (Transformation|GetWorldTransform (Variables|Default|GetDirectionalArrow)) "Undefined" "MultiplyWithRoot" 0 (Math|Conversions|ToFloat(Integer) (Variables|Default|GetStrenghtShoot)) (Variables|Trap|Crossbow|GetIn%20Lifespan) (Variables|Trap|Crossbow|GetMax%20Speed) (Variables|Trap|Crossbow|GetProjectile%20Gravity%20Scale) (Variables|Trap|Crossbow|GetBounciness) (Variables|Trap|Crossbow|GetAirFriction) (Variables|Trap|Crossbow|GetShould%20Bounce) (Variables|Trap|Crossbow|GetDamage) 0)
  (Variables|Default|SetbCharge false)
  (Variables|Default|SetStrenghtShoot 0)
  (Utilities|FlowControl|Delay (Variables|Default|GetTimeBetweenShoot))
  (Variables|Default|SetCanShoot true))

(event EventTick
  (params (DeltaSeconds :type Float%20%28single-precision%29))
  ;[0.126 0.126 0.126] Charge shoot
  (if (Variables|Default|GetbCharge)
    (if (< (Variables|Default|GetStrenghtShoot) (Variables|Trap|Crossbow|GetMax%20Speed))
      (Variables|Default|SetStrenghtShoot (+ (Variables|Trap|Crossbow|GetSpeedChargeShoot) (Variables|Default|GetStrenghtShoot))))))

(event EventChargeShot
  ;[0.126 0.126 0.126] Charge shoot
  (if (Variables|Default|GetCanShoot)
    (Variables|Default|SetCanShoot false)
    (Variables|Default|SetbCharge true)))

(event EventStopped
  ;[0.07187 0.07187 0.07187] Input
  (Class|Crossbow|ReleaseShot))

(event EventStarted
  ;[0.07187 0.07187 0.07187] Input
  (Class|Crossbow|ChargeShot))

(event Input|KeyboardEvents|O
  (params (Key :type Key%20Structure :default "None"))
  ;[0.07187 0.07187 0.07187] Input
  (:Pressed
    (Class|Crossbow|ChargeShot)))

(event Input|KeyboardEvents|P
  (params (Key :type Key%20Structure :default "None"))
  ;[0.07187 0.07187 0.07187] Input
  (:Pressed
    (Class|Crossbow|ReleaseShot)))

(fn ConstructionScript)