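; Trap enemy actor that reacts to nearby RogueCharacters and, when one touches its push zone, pushes the overlapping actors and destroys itself.
; A detection volume, scaled in the construction script, maintains a list of players around it.
; Each tick it selects a player from that list by a distance check, then sets location and look-at rotation, falling back to SearchMovement without a valid target.
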(event OnComponentBeginOverlap(PushZone)
  (params (OverlappedComponent :type Primitive%20Component%20Object%20Reference) (OtherActor :type Actor%20Object%20Reference) (OtherComp :type Primitive%20Component%20Object%20Reference) (OtherBodyIndex :type Integer) (bFromSweep :type Boolean) (SweepResult :type Hit%20Result%20Structure%20%28by%20ref%29))
  ;[0.1427 0.1427 0.1427] Push Player
  (Utilities|Casting|CastToRogueCharacter OtherActor)
  (Class|Enemy|Push (Collision|GetOverlappingActors (Variables|Default|GetPushZone) 0 :!class /Script/Engine.PrimitiveComponent))
  (Actor|DestroyActor))

(event OnComponentBeginOverlap(DetectPlayerAround)
  (params (OverlappedComponent :type Primitive%20Component%20Object%20Reference) (OtherActor :type Actor%20Object%20Reference) (OtherComp :type Primitive%20Component%20Object%20Reference) (OtherBodyIndex :type Integer) (bFromSweep :type Boolean) (SweepResult :type Hit%20Result%20Structure%20%28by%20ref%29))
  ;[0.09271 0.09271 0.09271] List PlayerAround
  (bind _asrogue_character (Utilities|Casting|CastToRogueCharacter OtherActor))
  (Utilities|Array|Add (Variables|Default|GetListPlayerAround) _asrogue_character))

(event OnComponentEndOverlap(DetectPlayerAround)
  (params (OverlappedComponent :type Primitive%20Component%20Object%20Reference) (OtherActor :type Actor%20Object%20Reference) (OtherComp :type Primitive%20Component%20Object%20Reference) (OtherBodyIndex :type Integer))
  ;[0.09271 0.09271 0.09271] List PlayerAround
  (bind _asrogue_character (Utilities|Casting|CastToRogueCharacter OtherActor))
  (Utilities|Array|RemoveItem (Variables|Default|GetListPlayerAround) _asrogue_character))

(event EventTick
  (params (DeltaSeconds :type Float%20%28single-precision%29))
  (bind _returnvalue (Transformation|GetActorLocation))
  (bind _returnvalue_2 (Transformation|GetActorLocation))
  ;[0.1594 0.1594 0.1594] Move and Rotate to Player
  (for _array_element (Variables|Default|GetListPlayerAround)
    (if (< (Variables|Default|GetDistancePlayerCloser) (Transformation|GetDistanceTo _array_element self))
      (bind _output_get (Variables|Default|SetPlayerCloser _array_element))))
  (Utilities|IsValid _output_get
    (:Is%20Valid
      (Transformation|SetActorLocationAndRotation (* (Math|Vector|Normalize (- _returnvalue _returnvalue_2)) (Variables|Enemy|GetMovementSpeed)) (Math|Rotator|FindLookatRotation _returnvalue _returnvalue_2)))
    (:Is%20Not%20Valid
      (Class|Enemy|SearchMovement DeltaSeconds))))

(fn ConstructionScript
  (bind _detectplayeraround (Variables|Default|GetDetectPlayerAround))
  (Transformation|SetWorldScale3D _detectplayeraround (* (Transformation|GetWorldScale _detectplayeraround) (Variables|Enemy|GetSizeBoxDetectingPlayer))))