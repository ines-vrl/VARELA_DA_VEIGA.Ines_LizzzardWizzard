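; Flamethrower trap that burns RogueCharacters through up to four directional flames, each enabled by its own flag.
; On BeginPlay it plays its skeletal animation and hides all flames, then after a delay sets visibility and query collision per side.
; Each collider's begin overlap deals damage and starts a looping timer that clears itself after one delayed second hit.
; All four sides share one victim reference and timer handle, so a new overlap overwrites both.
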(event OnComponentBeginOverlap(FireColliderNorth)
  (params (OverlappedComponent :type Primitive%20Component%20Object%20Reference) (OtherActor :type Actor%20Object%20Reference) (OtherComp :type Primitive%20Component%20Object%20Reference) (OtherBodyIndex :type Integer) (bFromSweep :type Boolean) (SweepResult :type Hit%20Result%20Structure%20%28by%20ref%29))
  (bind _asrogue_character (Utilities|Casting|CastToRogueCharacter OtherActor))
  (bind _output_get (Variables|Default|SetAs%20Rogue%20Character _asrogue_character))
  (Class|RogueCharacter|TakeDamage _output_get (Variables|Trap|FLameThrower|GetDamage))
  (bind _returnvalue (Utilities|Time|SetTimerbyEvent (delegate Custom|TakeDamage) (Variables|Trap|FLameThrower|GetDeltaTimeDamage) true))
  (Variables|Default|SetTimerFlame _returnvalue))

(event OnComponentBeginOverlap(FireColliderSouth)
  (params (OverlappedComponent :type Primitive%20Component%20Object%20Reference) (OtherActor :type Actor%20Object%20Reference) (OtherComp :type Primitive%20Component%20Object%20Reference) (OtherBodyIndex :type Integer) (bFromSweep :type Boolean) (SweepResult :type Hit%20Result%20Structure%20%28by%20ref%29))
  (bind _asrogue_character (Utilities|Casting|CastToRogueCharacter OtherActor))
  (bind _output_get (Variables|Default|SetAs%20Rogue%20Character _asrogue_character))
  (Class|RogueCharacter|TakeDamage _output_get (Variables|Trap|FLameThrower|GetDamage))
  (bind _returnvalue (Utilities|Time|SetTimerbyEvent (delegate Custom|CustomEvent) (Variables|Trap|FLameThrower|GetDeltaTimeDamage) true))
  (Variables|Default|SetTimerFlame _returnvalue))

(event OnComponentBeginOverlap(FlamecolliderWest)
  (params (OverlappedComponent :type Primitive%20Component%20Object%20Reference) (OtherActor :type Actor%20Object%20Reference) (OtherComp :type Primitive%20Component%20Object%20Reference) (OtherBodyIndex :type Integer) (bFromSweep :type Boolean) (SweepResult :type Hit%20Result%20Structure%20%28by%20ref%29))
  (bind _asrogue_character (Utilities|Casting|CastToRogueCharacter OtherActor))
  (bind _output_get (Variables|Default|SetAs%20Rogue%20Character _asrogue_character))
  (Class|RogueCharacter|TakeDamage _output_get (Variables|Trap|FLameThrower|GetDamage))
  (bind _returnvalue (Utilities|Time|SetTimerbyEvent (delegate Custom|CustomEvent_1) (Variables|Trap|FLameThrower|GetDeltaTimeDamage) true))
  (Variables|Default|SetTimerFlame _returnvalue))

(event OnComponentBeginOverlap(FlamecolliderEast)
  (params (OverlappedComponent :type Primitive%20Component%20Object%20Reference) (OtherActor :type Actor%20Object%20Reference) (OtherComp :type Primitive%20Component%20Object%20Reference) (OtherBodyIndex :type Integer) (bFromSweep :type Boolean) (SweepResult :type Hit%20Result%20Structure%20%28by%20ref%29))
  (bind _asrogue_character (Utilities|Casting|CastToRogueCharacter OtherActor))
  (bind _output_get (Variables|Default|SetAs%20Rogue%20Character _asrogue_character))
  (Class|RogueCharacter|TakeDamage _output_get (Variables|Trap|FLameThrower|GetDamage))
  (bind _returnvalue (Utilities|Time|SetTimerbyEvent (delegate Custom|CustomEvent_2) (Variables|Trap|FLameThrower|GetDeltaTimeDamage) true))
  (Variables|Default|SetTimerFlame _returnvalue))

(event Custom|CustomEvent_2
  (Class|RogueCharacter|TakeDamage (stale OnComponentBeginOverlap(FlamecolliderEast) _output_get) (Variables|Trap|FLameThrower|GetDamage))
  (Utilities|Time|ClearandInvalidateTimerbyHandle (Variables|Default|GetTimerFlame)))

(event Custom|TakeDamage
  (Class|RogueCharacter|TakeDamage (stale OnComponentBeginOverlap(FireColliderNorth) _output_get) (Variables|Trap|FLameThrower|GetDamage))
  (Utilities|Time|ClearandInvalidateTimerbyHandle (Variables|Default|GetTimerFlame)))

(event Custom|CustomEvent
  (Class|RogueCharacter|TakeDamage (stale OnComponentBeginOverlap(FireColliderSouth) _output_get) (Variables|Trap|FLameThrower|GetDamage))
  (Utilities|Time|ClearandInvalidateTimerbyHandle (Variables|Default|GetTimerFlame)))

(event Custom|CustomEvent_1
  (Class|RogueCharacter|TakeDamage (stale OnComponentBeginOverlap(FlamecolliderWest) _output_get) (Variables|Trap|FLameThrower|GetDamage))
  (Utilities|Time|ClearandInvalidateTimerbyHandle (Variables|Default|GetTimerFlame)))

(event EventBeginPlay
  (bind _sk_flamethrower (Variables|Default|GetSK_FlameThrower))
  (bind _frontflame (Variables|Trap|FLameThrower|ActiveFlame|GetFrontFlame))
  (bind _rightflame (Variables|Trap|FLameThrower|ActiveFlame|GetRightFlame))
  (bind _leftflame (Variables|Trap|FLameThrower|ActiveFlame|GetLeftFlame))
  (bind _backflame (Variables|Trap|FLameThrower|ActiveFlame|GetBackFlame))
  (bind _firecollidersouth (Variables|Default|GetFireColliderSouth))
  (bind _flamecolliderwest (Variables|Default|GetFlamecolliderWest))
  (bind _flamecollidereast (Variables|Default|GetFlamecolliderEast))
  (bind _firecollidernorth (Variables|Default|GetFireColliderNorth))
  (Components|Animation|PlayAnimation _sk_flamethrower 0 false)
  (Components|Timeline|SetPlayRate _sk_flamethrower (Variables|Trap|FLameThrower|GetSpeedAnimation))
  (Rendering|SetVisibility (Variables|Default|GetFlameNorth) false true)
  (Utilities|FlowControl|Delay (Variables|Trap|FLameThrower|GetTimeBeforeFlame))
  (Rendering|SetVisibility (Variables|Default|GetFlameSouth) _frontflame true)
  (if _frontflame
    (Collision|SetCollisionEnabled _firecollidersouth "QueryOnly")
    (else
      (Collision|SetCollisionEnabled _firecollidersouth "NoCollision")))
  (Rendering|SetVisibility (Variables|Default|GetFlameWest) _rightflame true)
  (if _rightflame
    (Collision|SetCollisionEnabled _flamecolliderwest "QueryOnly")
    (else
      (Collision|SetCollisionEnabled _flamecolliderwest "NoCollision")))
  (Rendering|SetVisibility (Variables|Default|GetFlameEast) _leftflame true)
  (if _leftflame
    (Collision|SetCollisionEnabled _flamecollidereast "QueryOnly")
    (else
      (Collision|SetCollisionEnabled _flamecollidereast "NoCollision")))
  (Rendering|SetVisibility (Variables|Default|GetFlameNorth) _backflame true)
  (if _backflame
    (Collision|SetCollisionEnabled _firecollidernorth "QueryOnly")
    (else
      (Collision|SetCollisionEnabled _firecollidernorth "NoCollision"))))

(fn ConstructionScript)