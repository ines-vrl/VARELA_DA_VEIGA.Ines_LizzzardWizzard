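; BP_Trap is a two-panel trapdoor that swings open when triggered through Started, then closes after a delay.
; OpenTrap rotates TrapLeft and TrapRight with MoveComponentTo, switching CollisionTrap off while open and back to query-only on closing.
; A CanOpen flag blocks retriggering until a cooldown ends, with a DoOnce path for non-reusable traps.
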(event EventOpenTrap
  (bind _timetoopentrap (Variables|Trap|Trap|GetTimetoOpenTrap))
  (bind _timetoopentrap_2 (Variables|Trap|Trap|GetTimetoOpenTrap))
  (if (Variables|Default|GetCanOpen)
    (Variables|Default|SetCanOpen false)
    (if (Variables|Trap|Trap|GetReusable)
      _
      (else
        (Utilities|FlowControl|DoOnce false
          (:Completed
            _))))
    (Utilities|FlowControl|Sequence
      (:then_0
        (Components|MoveComponentTo (Variables|Default|GetTrapRight) "0.000000,-50.000000,0.000000" "0.000000,0.000000,90.000000" false true _timetoopentrap true)
        (Collision|SetCollisionEnabled (Variables|Default|GetCollisionTrap) "NoCollision"))
      (:then_1
        (Components|MoveComponentTo (Variables|Default|GetTrapLeft) "0.000000,50.000000,0.000000" "0.000000,0.000000,-90.000000" false true _timetoopentrap true)
        (Utilities|FlowControl|Delay (Variables|Trap|Trap|GetTimeTrapOpen))
        (Utilities|FlowControl|Sequence
          (:then_0
            (Components|MoveComponentTo (Variables|Default|GetTrapRight) "0.000000,-50.000000,0.000000" "0, 0, 0" true false _timetoopentrap_2 true)
            (Collision|SetCollisionEnabled (Variables|Default|GetCollisionTrap) "QueryOnly"))
          (:then_1
            (Components|MoveComponentTo (Variables|Default|GetTrapLeft) "0.000000,50.000000,0.000000" "0, 0, 0" true false _timetoopentrap_2 true)
            (Utilities|FlowControl|Delay (Variables|Trap|Trap|GetTimeBeforeUseItAgain))
            (Variables|Default|SetCanOpen true)))))))

(event EventStarted
  (Class|Trap|OpenTrap))

(fn ConstructionScript)