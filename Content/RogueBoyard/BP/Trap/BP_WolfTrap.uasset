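; Bear trap actor that snaps on contact and damages player characters.
; The Started event arms it, and the first overlap with its detection box disarms it and plays the trap animation directly on the skeletal mesh.
; Any actor springs it, but only a BP_Character takes damage.
; The AnimStart and AnimEnd events are empty, and the BeginPlay anim-instance cast drives nothing.
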(event OnComponentBeginOverlap(BoxDetectionPlayer)
  (params (OverlappedComponent :type Primitive%20Component%20Object%20Reference) (OtherActor :type Actor%20Object%20Reference) (OtherComp :type Primitive%20Component%20Object%20Reference) (OtherBodyIndex :type Integer) (bFromSweep :type Boolean) (SweepResult :type Hit%20Result%20Structure%20%28by%20ref%29))
  (if (Variables|Default|GetTrapSet)
    (Variables|Default|SetTrapSet false)
    (Components|Animation|PlayAnimation (Variables|Default|GetBearTrap) "/Game/RogueBoyard/GA/Assets/Meshs/msh_Beartrap/BeartrapAnimOPN_Bones_Armature_ArmatureAction_001.BeartrapAnimOPN_Bones_Armature_ArmatureAction_001" false)
    (bind _asbp_character (Utilities|Casting|CastToBP_Character OtherActor))
    (Class|RogueCharacter|TakeDamage _asbp_character (Variables|Trap|WolfTrap|GetDamage))))

(event Custom|AnimStart)

(event Custom|AnimEnd)

(event EventBeginPlay
  (Utilities|Casting|CastToAB_BearTrap (Components|SkeletalMesh|GetAnimInstance (Variables|Default|GetBearTrap))))

(event EventStarted
  (Variables|Default|SetTrapSet true))

(fn ConstructionScript)