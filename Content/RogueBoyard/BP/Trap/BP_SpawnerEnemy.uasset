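; BP_SpawnerEnemy is a trap that spawns a batch of BP_Enemy actors at random points inside a box zone.
; The Started event or a Tab debug-style key press triggers it if CanUse is true, spawning NEnemyToSpawn enemies at once, then calling CoolDown.
; The construction script sizes the square ZoneSpawn box from SizeZoneSpawn.
; A Delay using TimeBetweenSpawn is left unconnected, so spawns are not staggered.
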(event EventStarted
  (bind _zonespawn (Variables|Default|GetZoneSpawn))
  (bind _returnvalue (Transformation|GetWorldLocation _zonespawn))
  (bind _returnvalue_2 (Components|Box|GetScaledBoxExtent _zonespawn))
  (if (Variables|Default|GetcanUse)
    (for _index (range 1 (Variables|Trap|SpawnerEnemy|GetNEnemyToSpawn))
      (Game|SpawnActorfromClass "/Game/RogueBoyard/BP/Trap/BP_Enemy.BP_Enemy_C" (Math|Transform|MakeTransform (Math|Random|RandomPointinBoundingBox (Math|Vector|MakeVector (.x _returnvalue) (.y _returnvalue) (.z _returnvalue)) (Math|Vector|MakeVector (.x _returnvalue_2) (.y _returnvalue_2) 0.0)) "0, 0, 0" "1.000000,1.000000,1.000000") "AlwaysSpawn" "OverrideRootScale" 0 0))
    (Class|RogueTrap|CoolDown 5.0)))

(event Input|KeyboardEvents|Tab
  (params (Key :type Key%20Structure :default "None"))
  (bind _zonespawn (Variables|Default|GetZoneSpawn))
  (bind _returnvalue (Transformation|GetWorldLocation _zonespawn))
  (bind _returnvalue_2 (Components|Box|GetScaledBoxExtent _zonespawn))
  (:Pressed
    (if (Variables|Default|GetcanUse)
      (for _index (range 1 (Variables|Trap|SpawnerEnemy|GetNEnemyToSpawn))
        (Game|SpawnActorfromClass "/Game/RogueBoyard/BP/Trap/BP_Enemy.BP_Enemy_C" (Math|Transform|MakeTransform (Math|Random|RandomPointinBoundingBox (Math|Vector|MakeVector (.x _returnvalue) (.y _returnvalue) (.z _returnvalue)) (Math|Vector|MakeVector (.x _returnvalue_2) (.y _returnvalue_2) 0.0)) "0, 0, 0" "1.000000,1.000000,1.000000") "AlwaysSpawn" "OverrideRootScale" 0 0))
      (Class|RogueTrap|CoolDown 5.0))))

(fn ConstructionScript
  (bind _sizezonespawn (Variables|Trap|SpawnerEnemy|GetSizeZoneSpawn))
  (Components|Box|SetBoxExtent (Variables|Default|GetZoneSpawn) (Math|Vector|MakeVector _sizezonespawn _sizezonespawn 32.0) true))