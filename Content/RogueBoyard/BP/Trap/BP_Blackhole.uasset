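; Black hole trap that pulls player characters caught inside its sphere zone toward it.
; Zone overlaps maintain the list of affected BP_Characters and toggle their IsInBlackHole flag.
; Once initialized, Tick scales each character's BuffInBlackHole and the strength passed to AttractPlayers by distance over zone radius, so both peak at the center and weaken toward the edge.
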(event OnComponentEndOverlap(Zone)
  (params (OverlappedComponent :type Primitive%20Component%20Object%20Reference) (OtherActor :type Actor%20Object%20Reference) (OtherComp :type Primitive%20Component%20Object%20Reference) (OtherBodyIndex :type Integer))
  (bind _asbp_character (Utilities|Casting|CastToBP_Character OtherActor))
  (Utilities|Array|RemoveItem (Variables|Default|GetListPlayer) _asbp_character)
  (Variables|/Script/RogueBoyard.RogueCharacter|SetbIsInBlackHole _asbp_character false))

(event OnComponentBeginOverlap(Zone)
  (params (OverlappedComponent :type Primitive%20Component%20Object%20Reference) (OtherActor :type Actor%20Object%20Reference) (OtherComp :type Primitive%20Component%20Object%20Reference) (OtherBodyIndex :type Integer) (bFromSweep :type Boolean) (SweepResult :type Hit%20Result%20Structure%20%28by%20ref%29))
  (bind _asbp_character (Utilities|Casting|CastToBP_Character OtherActor))
  (Utilities|Array|Add (Variables|Default|GetListPlayer) _asbp_character)
  (Variables|/Script/RogueBoyard.RogueCharacter|SetbIsInBlackHole _asbp_character true))

(event EventTick
  (params (DeltaSeconds :type Float%20%28single-precision%29))
  (if (Variables|Default|GetInitialized)
    (for _array_element (Variables|Default|GetListPlayer)
      (Variables|/Script/RogueBoyard.RogueCharacter|SetbuffInBlackHole _array_element (* (Variables|Default|GetAttractionForce) (Math|Float|Lerp 1e+01 2.1 (/ (Math|Vector|Distance(Vector) (Transformation|GetActorLocation _array_element) (Transformation|GetActorLocation)) (Components|Sphere|GetScaledSphereRadius (Variables|Default|GetZone))))))
      (Class|Blackhole|AttractPlayers (Math|Float|Lerp 1.0 0.0 (/ (Math|Vector|Distance(Vector) (Transformation|GetActorLocation _array_element) (Transformation|GetActorLocation)) (Components|Sphere|GetScaledSphereRadius (Variables|Default|GetZone)))) _array_element))))

(event EventInit
  (Variables|Default|SetInitialized true))

(fn ConstructionScript)