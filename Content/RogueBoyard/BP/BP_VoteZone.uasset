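; BP_VoteZone is a voting area with four trigger zones, P1 to P4, that tracks characters standing inside them.
; All four zones feed one shared overlap counter, which changes only for BP_Character actors.
; Each entry increments the counter, fires the player-enter event and prints a debug message.
; Each exit decrements it and fires the all-players-left event once the count reaches zero or below.
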(event OnComponentBeginOverlap(P1VoteZone)
  (params (OverlappedComponent :type Primitive%20Component%20Object%20Reference) (OtherActor :type Actor%20Object%20Reference) (OtherComp :type Primitive%20Component%20Object%20Reference) (OtherBodyIndex :type Integer) (bFromSweep :type Boolean) (SweepResult :type Hit%20Result%20Structure%20%28by%20ref%29))
  (Utilities|Casting|CastToBP_Character OtherActor)
  (Math|Integer|IncrementInt (Variables|Default|GetOverlappedCharacter)
    (:%20%20
      (Default|CallOnPlayerEnterZoneEvent)
      (Development|PrintString "PlayerEnteredVote"))))

(event OnComponentBeginOverlap(P2VoteZone)
  (params (OverlappedComponent :type Primitive%20Component%20Object%20Reference) (OtherActor :type Actor%20Object%20Reference) (OtherComp :type Primitive%20Component%20Object%20Reference) (OtherBodyIndex :type Integer) (bFromSweep :type Boolean) (SweepResult :type Hit%20Result%20Structure%20%28by%20ref%29))
  (Utilities|Casting|CastToBP_Character OtherActor)
  (Math|Integer|IncrementInt (Variables|Default|GetOverlappedCharacter)
    (:%20%20
      (Default|CallOnPlayerEnterZoneEvent)
      (Development|PrintString "PlayerEnteredVote"))))

(event OnComponentBeginOverlap(P3VoteZone)
  (params (OverlappedComponent :type Primitive%20Component%20Object%20Reference) (OtherActor :type Actor%20Object%20Reference) (OtherComp :type Primitive%20Component%20Object%20Reference) (OtherBodyIndex :type Integer) (bFromSweep :type Boolean) (SweepResult :type Hit%20Result%20Structure%20%28by%20ref%29))
  (Utilities|Casting|CastToBP_Character OtherActor)
  (Math|Integer|IncrementInt (Variables|Default|GetOverlappedCharacter)
    (:%20%20
      (Default|CallOnPlayerEnterZoneEvent)
      (Development|PrintString "PlayerEnteredVote"))))

(event OnComponentBeginOverlap(P4VoteZone)
  (params (OverlappedComponent :type Primitive%20Component%20Object%20Reference) (OtherActor :type Actor%20Object%20Reference) (OtherComp :type Primitive%20Component%20Object%20Reference) (OtherBodyIndex :type Integer) (bFromSweep :type Boolean) (SweepResult :type Hit%20Result%20Structure%20%28by%20ref%29))
  (Utilities|Casting|CastToBP_Character OtherActor)
  (Math|Integer|IncrementInt (Variables|Default|GetOverlappedCharacter)
    (:%20%20
      (Default|CallOnPlayerEnterZoneEvent)
      (Development|PrintString "PlayerEnteredVote"))))

(event OnComponentEndOverlap(P1VoteZone)
  (params (OverlappedComponent :type Primitive%20Component%20Object%20Reference) (OtherActor :type Actor%20Object%20Reference) (OtherComp :type Primitive%20Component%20Object%20Reference) (OtherBodyIndex :type Integer))
  (Utilities|Casting|CastToBP_Character OtherActor)
  (bind _result (Math|Integer|DecrementInt (Variables|Default|GetOverlappedCharacter))
    (:%20%20
      (if (<= _result 0)
        (Default|CallOnAllPlayersLeaveZoneEvent)))))

(event OnComponentEndOverlap(P2VoteZone)
  (params (OverlappedComponent :type Primitive%20Component%20Object%20Reference) (OtherActor :type Actor%20Object%20Reference) (OtherComp :type Primitive%20Component%20Object%20Reference) (OtherBodyIndex :type Integer))
  (Utilities|Casting|CastToBP_Character OtherActor)
  (bind _result (Math|Integer|DecrementInt (Variables|Default|GetOverlappedCharacter))
    (:%20%20
      (if (<= _result 0)
        (Default|CallOnAllPlayersLeaveZoneEvent)))))

(event OnComponentEndOverlap(P3VoteZone)
  (params (OverlappedComponent :type Primitive%20Component%20Object%20Reference) (OtherActor :type Actor%20Object%20Reference) (OtherComp :type Primitive%20Component%20Object%20Reference) (OtherBodyIndex :type Integer))
  (Utilities|Casting|CastToBP_Character OtherActor)
  (bind _result (Math|Integer|DecrementInt (Variables|Default|GetOverlappedCharacter))
    (:%20%20
      (if (<= _result 0)
        (Default|CallOnAllPlayersLeaveZoneEvent)))))

(event OnComponentEndOverlap(P4VoteZone)
  (params (OverlappedComponent :type Primitive%20Component%20Object%20Reference) (OtherActor :type Actor%20Object%20Reference) (OtherComp :type Primitive%20Component%20Object%20Reference) (OtherBodyIndex :type Integer))
  (Utilities|Casting|CastToBP_Character OtherActor)
  (bind _result (Math|Integer|DecrementInt (Variables|Default|GetOverlappedCharacter))
    (:%20%20
      (if (<= _result 0)
        (Default|CallOnAllPlayersLeaveZoneEvent)))))

(fn ConstructionScript)