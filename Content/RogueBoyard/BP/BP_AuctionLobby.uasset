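; BP_AuctionLobby is the auction lobby room, driving the door, camera and HUD when the room begins and ends.
; On BeginPlay it caches the first player's HUD_Rogue and, if that cast succeeds, the BP_Door found in the level.
; BeginRoom passes the room camera to the door, hides the title card and starts the room timer.
; EndRoom closes the door and ends both the room and vote timers.
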(event EventBeginRoom
  (Default|CESetCam (Variables|Default|GetDoor) (Variables|Default|GetRoomCamera))
  (Default|CEHideTitleCardSimon (Variables|Default|GetHUD))
  (Default|CEStartRoomTimer (Variables|Default|GetHUD) (Variables|Default|GetMaxRoomTime)))

(event EventBeginPlay
  (bind _ashud_rogue (Utilities|Casting|CastToHUD_Rogue (HUD|GetHUD (Game|GetPlayerController 0))))
  (Variables|Default|SetHUD _ashud_rogue)
  (bind _returnvalue (Actor|GetActorOfClass "/Game/RogueBoyard/Props/BP_Door.BP_Door_C"))
  (Variables|Default|SetDoor _returnvalue))

(event EventEndRoom
  (Default|CeCloseDoor (Variables|Default|GetDoor))
  (Default|CEEndRoomTimer (Variables|Default|GetHUD))
  (Default|CEEndVoteTimer (Variables|Default|GetHUD)))

(fn ConstructionScript)