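; BP_Levier is an interactable lever actor that animates its handle when a character uses it.
; Interact fires a pull event, where a timeline rotates the handle offset component's pitch; bell interaction is rejected.
; BeginPlay caches the first BP_Door found in the level, but the shown graphs never use that reference.
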(event Custom|CE_PullLever
  (bind _angle (Timeline|PullHandle Play)
    (:Update
      (Transformation|SetRelativeRotation (Variables|Default|GetOffsetHandle) (Math|Rotator|MakeRotator 0.0 _angle 0.0) false false))))

(event EventBeginPlay
  (bind _returnvalue (Actor|GetActorOfClass "/Game/GP/Blueprints/BP_Door.BP_Door_C"))
  (Variables|Default|SetDoor _returnvalue))

(event Collision|EventActorBeginOverlap
  (params (OtherActor :type Actor%20Object%20Reference)))

(event EventTick
  (params (DeltaSeconds :type Float%20%28single-precision%29)))

(fn ConstructionScript)

(fn Interact
  (params (Character :type Character%20Object%20Reference))
  (CallFunction|CEPullLever)
  (return true))

(fn InteractwithBell
  (params (Char :type BPA%20Buttler%20Object%20Reference))
  (return false))