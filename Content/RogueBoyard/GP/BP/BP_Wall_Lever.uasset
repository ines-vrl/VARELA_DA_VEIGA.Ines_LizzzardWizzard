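; BP_Wall_Lever is a wall lever that swings a door open when something overlaps its box.
; The overlap plays the Pull_Lever timeline to roll the lever, and each update calls Play on the OpenDoor timeline.
; OpenDoor lerps the relative rotation of the first Doors entry's actor toward that entry's angle.
; BeginPlay stores a found BP_Door in a separate DoorActor variable that the rotation does not read.
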(event OnComponentBeginOverlap(Box)
  (params (OverlappedComponent :type Primitive%20Component%20Object%20Reference) (OtherActor :type Actor%20Object%20Reference) (OtherComp :type Primitive%20Component%20Object%20Reference) (OtherBodyIndex :type Integer) (bFromSweep :type Boolean) (SweepResult :type Hit%20Result%20Structure%20%28by%20ref%29))
  (bind _doors (Variables|Default|GetDoors))
  (bind _output (Utilities|Array|Get(acopy) _doors))
  (bind (_dooractor _rotationangle) (Utilities|Struct|BreakS_Door _output))
  (bind _angle (Timeline|Pull_Lever Play)
    (:Update
      (Transformation|SetRelativeRotation (Variables|Default|GetLeverOffset) (Math|Rotator|MakeRotator _angle 0.0 0.0) false false)
      (bind _newtrack_0 (Timeline|OpenDoor Play)
        (:Update
          (Transformation|SetActorRelativeRotation _dooractor (Math|Rotator|Lerp(Rotator) "0, 0, 0" _rotationangle _newtrack_0)))))))

(event EventBeginPlay
  (bind _returnvalue (Actor|GetActorOfClass "/Game/RogueBoyard/GP/BP/BP_Door.BP_Door_C"))
  (Variables|Default|SetDoorActor _returnvalue))

(fn ConstructionScript)