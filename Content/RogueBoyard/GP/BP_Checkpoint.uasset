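; BP_Checkpoint is a one-time checkpoint actor that records a position for the player's first-person character.
; On BeginPlay it casts player 0's character to BP_FirstPersonCharacter and caches it.
; When that character begins overlapping the Box component, the box's world location is written to the character's CheckpointPos, and a HasChecked flag prevents it from triggering again.
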(event OnComponentBeginOverlap(Box)
  (params (OverlappedComponent :type Primitive%20Component%20Object%20Reference) (OtherActor :type Actor%20Object%20Reference) (OtherComp :type Primitive%20Component%20Object%20Reference) (OtherBodyIndex :type Integer) (bFromSweep :type Boolean) (SweepResult :type Hit%20Result%20Structure%20%28by%20ref%29))
  (bind _bp_character (Variables|Default|GetBP_Character))
  (if (== OtherActor _bp_character)
    (if (not (Variables|Default|GethasChecked))
      (Variables|/Game/FirstPerson/Blueprints/BP_FirstPersonCharacter.BP_FirstPersonCharacter_C|SetCheckpointPos _bp_character (Transformation|GetWorldLocation (Variables|Default|GetBox)))
      (Variables|Default|SethasChecked true))))

(event EventBeginPlay
  (bind _asbp_first_person_character (Utilities|Casting|CastToBP_FirstPersonCharacter (Game|GetPlayerCharacter 0)))
  (Variables|Default|SetBP_Character _asbp_first_person_character))

(fn ConstructionScript)