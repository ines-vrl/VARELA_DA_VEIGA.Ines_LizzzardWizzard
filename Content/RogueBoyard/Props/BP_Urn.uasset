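; BP_Urn is an interactable urn prop where characters spend coins to add bids, shown as vote progress.
; On BeginPlay it tints the progress bar in its widget component with the urn's color.
; Each interaction spawns a scaled-down BP_FRCoin that only overlaps one custom channel, adds a bid and spends one coin from the character's purse.
; It then sets the bar to bids over MaxBids and plays a Wwise coin sound.
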(event EventInteract
  (params (Character :type BP%20Character%20Object%20Reference))
  (bind _returnvalue (Game|SpawnActorfromClass "/Game/RogueBoyard/Props/BP_FRCoin.BP_FRCoin_C" (Transformation|GetWorldTransform (Variables|Default|GetScene)) "Undefined" "MultiplyWithRoot" 0 0))
  (Transformation|SetActorScale3D _returnvalue "0.750000,0.750000,0.750000")
  (Collision|SetCollisionResponsetoAllChannels (Variables|/Game/RogueBoyard/Props/BP_FRCoin.BP_FRCoin_C|GetCylinder _returnvalue) "ECR_Ignore")
  (Collision|SetCollisionResponsetoChannel (Variables|/Game/RogueBoyard/Props/BP_FRCoin.BP_FRCoin_C|GetCylinder _returnvalue) "ECC_GameTraceChannel1" "ECR_Overlap")
  (Class|RogueAuctionUrn|AddBid)
  (Class|RoguePurse|Spend (Variables|/Script/RogueBoyard.RogueCharacter|GetPurse Character) 1)
  (Progress|SetPercent (Variables|/Game/RogueBoyard/UMG/Widgets/WBP_UrnProgressBar.WBP_UrnProgressBar_C|GetVoteProgression (Variables|Default|GetAs%20WBP%20Urn%20Progress%20Bar)) (/ (Class|RogueAuctionUrn|GetBids) (Variables|Default|GetMaxBids)))
  (Class|AkGameplayStatics|PostEvent "/Game/WwiseAudio/Events/Default_Work_Unit/Items/Coin/Play_SFX_Item_Coins_Buying.Play_SFX_Item_Coins_Buying"))

(event EventBeginPlay
  (bind _aswbp_urn_progress_bar (Utilities|Casting|CastToWBP_UrnProgressBar (UserInterface|GetWidget (Variables|Default|GetWidget))))
  (bind _output_get (Variables|Default|SetAs%20WBP%20Urn%20Progress%20Bar _aswbp_urn_progress_bar))
  (Class|ProgressBar|SetFillColorandOpacity (Variables|/Game/RogueBoyard/UMG/Widgets/WBP_UrnProgressBar.WBP_UrnProgressBar_C|GetVoteProgression _output_get) (Variables|Default|GetColor)))

(fn ConstructionScript)