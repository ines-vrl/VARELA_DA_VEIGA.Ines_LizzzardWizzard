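; Door prop for RogueBoyard that positions itself in front of a room camera, then animates open.
; Setting the camera starts a looping timer that keeps the door at a fixed distance along the camera's view with matching rotation, until the placement time elapses and opening is triggered.
; Open and close events each play a skeletal mesh animation and run a timeline that sets location from offsets along the camera's forward axis.
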(event Custom|CE_OpenDoor
  (bind _returnvalue (Transformation|GetActorLocation))
  (Components|Animation|PlayAnimation (Variables|Default|GetSkeletalMesh) "/Game/RogueBoyard/GA/Assets/Meshs/Door/Animation_Porte_Montage.Animation_Porte_Montage" false)
  (Development|PrintString "Open")
  (Variables|Default|SetStartPos _returnvalue)
  (Variables|Default|SetEndPos (- _returnvalue (* (Math|Vector|GetForwardVector (Transformation|GetActorRotation (Variables|Default|GetRoomCamera))) 25)))
  (bind _speed (Timeline|_Open PlayFromStart)
    (:Update
      (Transformation|SetActorLocation (Math|Vector|Lerp(Vector) (Variables|Default|GetStartPos) (Variables|Default|GetEndPos) _speed) false false))))

(event Custom|Ce_CloseDoor
  (Components|Animation|PlayAnimation (Variables|Default|GetSkeletalMesh) "/Game/RogueBoyard/GA/Assets/Meshs/Door/Animation_PorteClose_Montage.Animation_PorteClose_Montage" false)
  (Development|PrintString "Close")
  (Variables|Default|SetStartPoseClose (Variables|Default|GetStartPos))
  (Variables|Default|SetEndPos (- (Transformation|GetActorLocation) (* (Math|Vector|GetForwardVector (Transformation|GetActorRotation (Variables|Default|GetRoomCamera))) -25)))
  (bind _speed (Timeline|Timeline PlayFromStart)
    (:Update
      (Transformation|SetActorLocation (Math|Vector|Lerp(Vector) (Variables|Default|GetStartPos) (Variables|Default|GetEndPos) _speed) false false))))

(event Custom|CE_SetCam
  (params (Camera :type Camera%20Actor%20Object%20Reference))
  (Variables|Default|SetRoomCamera Camera)
  (Development|PrintString "SetCam")
  (bind _returnvalue (Utilities|Time|SetTimerbyFunctionName 0 "PlaceDoor" 0.05 true))
  (Variables|Default|SetTimerPlaceDoor _returnvalue))

(event EventBeginPlay
  (bind _asgm_rogue (Utilities|Casting|CastToGM_Rogue (Game|GetGameMode)))
  (Variables|Default|SetGM _asgm_rogue))

(event Collision|EventActorBeginOverlap
  (params (OtherActor :type Actor%20Object%20Reference)))

(fn ConstructionScript)

(fn PlaceDoor
  (bind _roomcamera (Variables|Default|GetRoomCamera))
  (bind _returnvalue (Transformation|GetActorRotation _roomcamera))
  (bind (_roll _pitch _yaw) (Math|Rotator|BreakRotator _returnvalue))
  (Variables|Default|SetCurrentTime (+ (Variables|Default|GetCurrentTime) 0.05))
  (if (>= (Variables|Default|GetCurrentTime) (Variables|Default|GetTimeToPlace))
    (CallFunction|CEOpenDoor)
    (Utilities|Time|ClearandInvalidateTimerbyHandle (Variables|Default|GetTimerPlaceDoor))
    (Variables|Default|SetTimerPlaceDoor "")
    (Variables|Default|SetCurrentTime 0.0)
    (else
      (Transformation|SetActorLocation (+ (Transformation|GetActorLocation _roomcamera) (* (Math|Vector|GetForwardVector _returnvalue) (Variables|Default|GetDoorDistToCam))) false true)
      (Transformation|SetActorRotation (Math|Rotator|MakeRotator _roll _pitch _yaw)))))