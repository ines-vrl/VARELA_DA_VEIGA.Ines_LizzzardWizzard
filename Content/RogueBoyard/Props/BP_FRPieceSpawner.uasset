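; BP_FRPieceSpawner is a prop actor that emits a requested number of BP_FRCoin pickups from its own location.
; CE_SpawnCoins stores the count and starts a self-calling loop that spawns a coin, waits briefly, decrements the counter and posts a Wwise coin sound.
; Each coin gets a random rotation and always spawns regardless of collision, producing a staggered burst.
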(event Custom|CE_SpawnCoin
  (Game|SpawnActorfromClass "/Game/RogueBoyard/Props/BP_FRCoin.BP_FRCoin_C" (Math|Transform|MakeTransform (Transformation|GetActorLocation) (Math|Random|RandomRotator true) "1.000000,1.000000,1.000000") "AlwaysSpawn" "MultiplyWithRoot" 0 0))

(event Custom|CE_SpawnCoins
  (params (Nb :type Integer))
  (Variables|Default|SetCoinsLeft Nb)
  (CallFunction|CECoinSpawnLoop))

(event Custom|CE_CoinSpawnLoop
  (if (not (<= (Variables|Default|GetCoinsLeft) 0))
    (CallFunction|CESpawnCoin)
    (Utilities|FlowControl|Delay 0.1)
    (Math|Integer|DecrementInt (Variables|Default|GetCoinsLeft)
      (:%20%20
        (Class|AkGameplayStatics|PostEvent "/Game/WwiseAudio/Events/Default_Work_Unit/Items/Coin/Play_SFX_Item_Coins_Get.Play_SFX_Item_Coins_Get")
        (CallFunction|CECoinSpawnLoop)))))

(fn ConstructionScript)