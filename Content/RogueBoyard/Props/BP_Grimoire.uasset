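; BP_Grimoire is a prop that a RogueCharacter picks up by touch and loses when pushed.
; Overlapping the root while grounded calls SwitchOwner with that character, clears Grounded and binds to the new owner's pushed event.
; When that event fires, it marks itself grounded again, unbinds and calls SwitchOwner with no character, releasing it for the next pickup.
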(event OnComponentBeginOverlap(Root)
  (params (OverlappedComponent :type Primitive%20Component%20Object%20Reference) (OtherActor :type Actor%20Object%20Reference) (OtherComp :type Primitive%20Component%20Object%20Reference) (OtherBodyIndex :type Integer) (bFromSweep :type Boolean) (SweepResult :type Hit%20Result%20Structure%20%28by%20ref%29))
  (bind _asrogue_character (Utilities|Casting|CastToRogueCharacter OtherActor))
  (if (Variables|Default|GetbGrounded)
    (Class|RogueGrimoire|SwitchOwner _asrogue_character)
    (Variables|Default|SetbGrounded false)
    (EventDispatchers|AssignOnCharacterPushedEvent (Variables|Default|GetCurrentOwner) (delegate Custom|OnOwnerPushed))))

(event Custom|OnOwnerPushed
  (Variables|Default|SetbGrounded true)
  (EventDispatchers|UnbindEventfromOnCharacterPushedEvent (Variables|Default|GetCurrentOwner) (delegate Custom|OnOwnerPushed))
  (Class|RogueGrimoire|SwitchOwner))

(fn ConstructionScript)