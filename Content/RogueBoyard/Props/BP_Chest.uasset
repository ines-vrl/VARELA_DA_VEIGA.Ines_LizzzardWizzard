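; BP_Chest is an interactable treasure chest prop that rewards the interacting character with coins.
; Its Interact event runs only once, guarded by an Interacted flag.
; On use it plays the opening montage on the skeletal mesh, spawns a Niagara effect at a scene component's location, adds the coin reward to the character's Purse and posts a Wwise open sound.
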(event EventBeginPlay)

(event Collision|EventActorBeginOverlap
  (params (OtherActor :type Actor%20Object%20Reference)))

(event EventTick
  (params (DeltaSeconds :type Float%20%28single-precision%29)))

(event EventInteract
  (params (Character :type BP%20Character%20Object%20Reference))
  (if (not (Variables|Default|GetInteracted))
    (Variables|Default|SetInteracted true)
    (Components|Animation|PlayAnimation (Variables|Default|GetSkeletalMesh) "/Game/RogueBoyard/GA/Assets/Meshs/msh_Chest/ChestAnim_Anim_Montage.ChestAnim_Anim_Montage" false)
    (Niagara|SpawnSystematLocation "/Game/RogueBoyard/VFX/NS_Chest.NS_Chest" (Transformation|GetWorldLocation (Variables|Default|GetScene)))
    (Class|RoguePurse|Earn (Variables|/Script/RogueBoyard.RogueCharacter|GetPurse Character) (Variables|Default|GetCoinsWon))
    (Class|AkGameplayStatics|PostEvent "/Game/WwiseAudio/Events/Default_Work_Unit/Items/Play_Chest_Open.Play_Chest_Open")))

(fn ConstructionScript)