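; BP_Statue is a statue actor that plays a colored Niagara effect and then shows its mesh.
; On BeginPlay it attaches NS_Statue to the StaticMesh, passing in that mesh and the Color variable, then makes the mesh visible after a two-second delay.
; BeginAnim replays this sequence for a matching PlayerIndex, but its binding to the local multiplayer player-joined event is disconnected and never runs.
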(event Custom|BeginAnim
  (params (PlayerIndex :type Integer))
  (if (== PlayerIndex (Variables|Default|GetPlayerIndex))
    (bind _returnvalue (Niagara|SpawnSystemAttached "/Game/RogueBoyard/VFX/NS_Statue.NS_Statue" (Variables|Default|GetStaticMesh) "None" "0, 0, 0" "0, 0, 0" "KeepRelativeOffset" false))
    (Class|NiagaraComponent|SetVariableStaticMesh _returnvalue "Mesh" (Variables|/Script/Engine.StaticMeshComponent|GetStaticMesh (Variables|Default|GetStaticMesh)))
    (Niagara|SetNiagaraVariable(LinearColor) _returnvalue "Color" (Math|Conversions|ToLinearColor(Color) (Variables|Default|GetColor)))
    (Utilities|FlowControl|Delay 2.0)
    (Rendering|SetVisibility (Variables|Default|GetStaticMesh) true false)))

(event EventBeginPlay
  (bind _returnvalue (Niagara|SpawnSystemAttached "/Game/RogueBoyard/VFX/NS_Statue.NS_Statue" (Variables|Default|GetStaticMesh) "None" "0, 0, 0" "0, 0, 0" "KeepRelativeOffset" false))
  (Class|NiagaraComponent|SetVariableStaticMesh _returnvalue "Mesh" (Variables|/Script/Engine.StaticMeshComponent|GetStaticMesh (Variables|Default|GetStaticMesh)))
  (Niagara|SetNiagaraVariable(LinearColor) _returnvalue "Color" (Math|Conversions|ToLinearColor(Color) (Variables|Default|GetColor)))
  (Utilities|FlowControl|Delay 2.0)
  (Rendering|SetVisibility (Variables|Default|GetStaticMesh) true false))

(fn ConstructionScript)