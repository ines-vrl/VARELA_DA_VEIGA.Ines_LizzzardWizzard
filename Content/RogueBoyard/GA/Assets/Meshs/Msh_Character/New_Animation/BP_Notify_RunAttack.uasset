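; Anim notify for the run attack that spawns a player-colored push effect on the character.
; It destroys the character's existing FX component if valid, then spawns the NS_Push Niagara system at the CentreAureole socket's location and yaw.
; The player index selects a DT_Character row, whose player color is passed to the system's PartColor variable.
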(fn ReceivedNotify
  (params (MeshComp :type Skeletal%20Mesh%20Component%20Object%20Reference) (Animation :type Anim%20Sequence%20Base%20Object%20Reference) (EventReference :type Anim%20Notify%20Event%20Reference%20Structure%20%28by%20ref%29))
  (bind _asbp_character (Utilities|Casting|CastToBP_Character (Components|GetOwner MeshComp)))
  (Utilities|IsValid (Variables|/Game/RogueBoyard/Core/BP_Character.BP_Character_C|GetFX _asbp_character)
    (:Is%20Valid
      (Components|DestroyComponent (Variables|/Game/RogueBoyard/Core/BP_Character.BP_Character_C|GetFX _asbp_character)))
    (:Is%20Not%20Valid
      _))
  (bind _returnvalue (Niagara|SpawnSystematLocation "/Game/RogueBoyard/VFX/Systems/Player/NS_Push.NS_Push" (Transformation|GetSocketLocation (Variables|/Script/Engine.Character|GetMesh _asbp_character) "CentreAureole") (Math|Rotator|MakeRotator 0.0 0.0 (.yaw (Transformation|GetSocketRotation (Variables|/Script/Engine.Character|GetMesh _asbp_character) "CentreAureole")))))
  (bind _returnvalue_2 (Utilities|GetDataTableRow "/Game/RogueBoyard/Characters/DT_Character.DT_Character" (Utilities|Select :Index (Variables|/Script/RogueBoyard.RogueCharacter|GetPlayerIndex _asbp_character) :Option%200 "J1" :Option%201 "J2" :Option%202 "J3" :Option%203 "J4"))
    (:then
      (Niagara|SetNiagaraVariable(LinearColor) _returnvalue "PartColor" (Math|Conversions|ToLinearColor(Color) (.player_color _returnvalue_2)))
      (return false))))