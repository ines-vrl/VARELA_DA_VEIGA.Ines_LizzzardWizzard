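; Player character for RogueBoyard that routes move, dash, push, interact and resurrect inputs into a state machine and resets its camera on each new room.
; Looping timers drive dash and push cooldowns and the push charge, which slows movement and scales force.
; A successful full-charge push adds camera shake and a global time-dilation freeze.
; Interact also buys shop items and bids on auction urns from the purse, and Paralysis applies stun.
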(event Custom|CE_OnNextRoom
  ;[1 1 1] Begin Play
  (Class|RogueCharacter|SetCamera))

(event Custom|FullCharged
  ;[1 0.2747 0.2687] Push
  (bind _returnvalue (Class|RogueCharacterStatePushing|Pushing (Variables|Default|GetRogueCharacterStatePushing) (Collision|GetOverlappingActors (Variables|Default|GetBox) 0 :!class /Script/Engine.PrimitiveComponent) (Variables|Pushing|GetForcePush)))
  (if _returnvalue
    (Camera|PlayWorldCameraShake "/Game/RogueBoyard/Core/Shaking/ShakeAfterPushing.ShakeAfterPushing_C" (Transformation|GetActorLocation (Variables|/Script/RogueBoyard.RogueRoom|GetRoomCamera (Variables|/Script/RogueBoyard.RogueGameMode|GetActiveRoom (Variables|Default|GetGameMode)))) 0.0 5e+02)
    (Utilities|FlowControl|Delay 0.25)
    (Utilities|Time|SetGlobalTimeDilation 0.05)
    (Utilities|FlowControl|Delay (Variables|Pushing|GetFreezeScreenDuration))
    (Utilities|Time|SetGlobalTimeDilation 1.0))
  (Variables|Pushing|SetForcePush 0.0)
  (Variables|Default|SetspeedNerfPrivate 1.0)
  (Variables|Pushing|SetTimerPushing "")
  (Variables|Pushing|SetTimeForce 0.0)
  (bind _returnvalue_2 (Utilities|Time|SetTimerbyFunctionName 0 "TimerPushSetting" 0.1 true))
  (Variables|Pushing|SetTimerPushCooldown _returnvalue_2))

(event Input|EnhancedActionEvents|EnhancedInputActionIA_Dash
  (params (ActionValue :type Boolean) (ElapsedSeconds :type Float%20%28double-precision%29) (TriggeredSeconds :type Float%20%28double-precision%29) (InputAction :type Input%20Action%20Object%20Reference :default "/Game/RogueBoyard/Inputs/InputDataPlaytest/IA_Dash.IA_Dash"))
  ;[0.1836 0.2918 1] Dash
  (:Started
    (if (and (AI|Components|NavMovement|IsMovingonGround (Variables|Character|GetCharacterMovement)) (not (Utilities|Time|IsTimerActivebyHandle (Variables|Default|GetTimerDash))))
      (Variables|Dash|SetStartDash (Transformation|GetActorLocation))
      (bind _returnvalue (Class|RogueCharacterState|Dash (Variables|/Script/RogueBoyard.RogueCharacterStateMachine|GetCurrentState (Variables|Default|GetStateMachine)) (.y (stale Input|EnhancedActionEvents|EnhancedInputActionIA_PTMoves ActionValue)) (.x (stale Input|EnhancedActionEvents|EnhancedInputActionIA_PTMoves ActionValue))))
      (Variables|Dash|SetDashed _returnvalue)
      (if (not (and _returnvalue (>= (Variables|Default|GetTimeDash) 0.1)))
        (bind _returnvalue_2 (Utilities|Time|SetTimerbyFunctionName 0 "TimerDashSetting" 0.1 true))
        (Variables|Default|SetTimerDash _returnvalue_2)))))

(event Input|EnhancedActionEvents|EnhancedInputActionIA_PTMoves
  (params (ActionValue :type Vector%202D%20Structure) (ElapsedSeconds :type Float%20%28double-precision%29) (TriggeredSeconds :type Float%20%28double-precision%29) (InputAction :type Input%20Action%20Object%20Reference :default "/Game/RogueBoyard/Inputs/InputDataPlaytest/IA_PTMoves.IA_PTMoves"))
  (bind _returnvalue (Transformation|GetVelocity))
  (bind _statemachine (Variables|Default|GetStateMachine))
  (bind _forwardvector (Variables|Default|GetForwardVector))
  (bind _speednerfprivate (Variables|Default|GetspeedNerfPrivate))
  ;[0.4104 1 0.4759] Movements
  (:Triggered
    (bind _newparam (CallFunction|Threshold (.x ActionValue) (.y ActionValue)))
    (if (or _newparam (not (AI|Components|NavMovement|IsMovingonGround (Variables|Character|GetCharacterMovement))))
      (Variables|/Script/RogueBoyard.RogueCharacterStateMachine|SetSticks _statemachine (Math|Vector|MakeVector 0.0 0.0 0.0) :!label _label)
      (else
        (Variables|/Script/RogueBoyard.RogueCharacterStateMachine|SetSticks _statemachine (Math|Vector|MakeVector (.x ActionValue) (.y ActionValue) (.z (Transformation|GetVelocity))))
        (Class|RogueCharacterState|Movement (Variables|/Script/RogueBoyard.RogueCharacterStateMachine|GetCurrentState _statemachine) (* (.x ActionValue) _speednerfprivate) (* (.y ActionValue) _speednerfprivate))
        (if (or (!= (.x _returnvalue) 0.0) (!= (.y _returnvalue) 0.0))
          (Transformation|SetWorldRotation (Variables|Character|GetMesh) (Math|Rotator|MakeRotfromX (Math|Vector|MakeVector (.y _forwardvector) (* (.x _forwardvector) -1.0) (.z _forwardvector))) false false)))))
  (:Completed
    (goto _label)))

(event Input|EnhancedActionEvents|EnhancedInputActionIA_Interact
  (params (ActionValue :type Boolean) (ElapsedSeconds :type Float%20%28double-precision%29) (TriggeredSeconds :type Float%20%28double-precision%29) (InputAction :type Input%20Action%20Object%20Reference :default "/Game/RogueBoyard/Inputs/InputDataPlaytest/IA_Interact.IA_Interact"))
  ;[1 1 1] Interact / Shop
  (:Started
    (bind _returnvalue (Class|RogueCharacterState|Interact (Variables|/Script/RogueBoyard.RogueCharacterStateMachine|GetCurrentState (Variables|Default|GetStateMachine))))
    (for _array_element _returnvalue
      (if (Utilities|DoesObjectImplementInterface _array_element "/Game/RogueBoyard/BP/I_Interactable.I_Interactable_C")
        (Class|IInteractable|Interact(Message) _array_element)))
    (CallFunction|TryBuyItem)
    (CallFunction|TryPayUrn)))

(event Input|EnhancedActionEvents|EnhancedInputActionIA_Push
  (params (ActionValue :type Boolean) (ElapsedSeconds :type Float%20%28double-precision%29) (TriggeredSeconds :type Float%20%28double-precision%29) (InputAction :type Input%20Action%20Object%20Reference :default "/Game/RogueBoyard/Inputs/InputDataPlaytest/IA_Push.IA_Push"))
  (bind _roguecharacterstatepushing (Variables|Default|GetRogueCharacterStatePushing))
  ;[1 0.2747 0.2687] Push
  (:Started
    (if (not (Utilities|Time|IsValidTimerHandle (Variables|Pushing|GetTimerPushCooldown)))
      (Class|RogueCharacterState|Push (Variables|/Script/RogueBoyard.RogueCharacterStateMachine|GetCurrentState (Variables|Default|GetStateMachine)))
      (bind _returnvalue (Utilities|Time|SetTimerbyFunctionName 0 "SetForcePush" 0.1 true))
      (Variables|Pushing|SetTimerPushing _returnvalue)
      (Variables|Default|SetspeedNerfPrivate (Variables|Default|GetSpeedNerf))
      (bind _returnvalue_2 (Niagara|SpawnSystemAttached "/Game/RogueBoyard/VFX/Systems/Player/NS_PlayerCharge.NS_PlayerCharge" (Variables|Character|GetMesh) "CentreAureole" "0, 0, 0" "0, 0, 0" "KeepRelativeOffset" false))
      (Variables|Default|SetFX _returnvalue_2)))
  (:Completed
    (if (Utilities|Time|IsValidTimerHandle (Variables|Pushing|GetTimerPushing))
      (Utilities|Time|ClearandInvalidateTimerbyHandle (Variables|Pushing|GetTimerPushing))
      (if (<= (Variables|Pushing|GetTimeForce) (Variables|/Script/RogueBoyard.RogueCharacterStatePushing|GetTimeMin _roguecharacterstatepushing))
        (Variables|Pushing|SetTimeForce (Variables|/Script/RogueBoyard.RogueCharacterStatePushing|GetMinForce _roguecharacterstatepushing)))
      (Class|RogueCharacterStatePushing|Pushing (Variables|Default|GetRogueCharacterStatePushing) (Collision|GetOverlappingActors (Variables|Default|GetBox) 0 :!class /Script/Engine.PrimitiveComponent) (Variables|Pushing|GetForcePush))
      (Variables|Pushing|SetForcePush 0.0)
      (Variables|Default|SetspeedNerfPrivate 1.0)
      (Variables|Pushing|SetTimerPushing "")
      (Variables|Pushing|SetTimeForce 0.0)
      (bind _returnvalue_3 (Utilities|Time|SetTimerbyFunctionName 0 "TimerPushSetting" 0.1 true))
      (Variables|Pushing|SetTimerPushCooldown _returnvalue_3))))

(event Input|EnhancedActionEvents|EnhancedInputActionIA_Resurect_1
  (params (ActionValue :type Boolean) (ElapsedSeconds :type Float%20%28double-precision%29) (TriggeredSeconds :type Float%20%28double-precision%29) (InputAction :type Input%20Action%20Object%20Reference :default "/Game/RogueBoyard/Inputs/InputDataPlaytest/IA_Resurect_1.IA_Resurect_1"))
  ;[1 0.8821 0.3875] Ressurect
  (if (and ActionValue (stale Input|EnhancedActionEvents|EnhancedInputActionIA_Resurect_2 ActionValue))
    (Class|RogueCharacterState|Resurrect (Variables|/Script/RogueBoyard.RogueCharacterStateMachine|GetCurrentState (Variables|Default|GetStateMachine)))
    (bind _asrogue_character_state_dead (Utilities|Casting|CastToRogueCharacterStateDead (Variables|/Script/RogueBoyard.RogueCharacterStateMachine|GetCurrentState (Variables|Default|GetStateMachine))))
    (Components|Animation|PlayAnimation (Variables|Character|GetMesh) (Variables|/Script/RogueBoyard.RogueCharacterStateDead|GetResurectMontage _asrogue_character_state_dead) false)))

(event Input|EnhancedActionEvents|EnhancedInputActionIA_Resurect_2
  (params (ActionValue :type Boolean) (ElapsedSeconds :type Float%20%28double-precision%29) (TriggeredSeconds :type Float%20%28double-precision%29) (InputAction :type Input%20Action%20Object%20Reference :default "/Game/RogueBoyard/Inputs/InputDataPlaytest/IA_Resurect_2.IA_Resurect_2"))
  ;[1 0.8821 0.3875] Ressurect
  (if (and (stale Input|EnhancedActionEvents|EnhancedInputActionIA_Resurect_1 ActionValue) ActionValue)
    (Class|RogueCharacterState|Resurrect (Variables|/Script/RogueBoyard.RogueCharacterStateMachine|GetCurrentState (Variables|Default|GetStateMachine)))
    (bind _asrogue_character_state_dead (Utilities|Casting|CastToRogueCharacterStateDead (Variables|/Script/RogueBoyard.RogueCharacterStateMachine|GetCurrentState (Variables|Default|GetStateMachine))))
    (Components|Animation|PlayAnimation (Variables|Character|GetMesh) (Variables|/Script/RogueBoyard.RogueCharacterStateDead|GetResurectMontage _asrogue_character_state_dead) false)))

(event Input|EnhancedActionEvents|EnhancedInputActionIA_Power
  (params (ActionValue :type Boolean) (ElapsedSeconds :type Float%20%28double-precision%29) (TriggeredSeconds :type Float%20%28double-precision%29) (InputAction :type Input%20Action%20Object%20Reference :default "/Game/RogueBoyard/Inputs/InputDataPlaytest/IA_Power.IA_Power"))
  ;[0.3397 1 0.9302] Use Item
  (:Started
    (Class|RogueItemComponent|UseItem (Variables|Default|GetUsableItem))))

(event EventBeginPlay
  ;[1 1 1] Begin Play
  (bind _asgm_rogue (Utilities|Casting|CastToGM_Rogue (Game|GetGameMode)))
  (Variables|Default|SetGameMode _asgm_rogue)
  (EventDispatchers|AssignOnNextRoomEvent (Subsystems|GetRogueRoomSubsystem) (delegate Custom|CE_OnNextRoom))
  (Variables|Default|SetspeedNerfPrivate 1.0))

(event EventTick
  (params (DeltaSeconds :type Float%20%28single-precision%29))
  (bind _charactermovement (Variables|Character|GetCharacterMovement))
  (if (Variables|Dash|GetDashed)
    (if (>= (Math|Vector|VectorLength (- (Transformation|GetActorLocation) (Variables|Dash|GetStartDash))) (Variables|Dash|GetDashDistanceMax))
      (Variables|/Script/Engine.MovementComponent|SetVelocity _charactermovement (/ (Variables|/Script/Engine.MovementComponent|GetVelocity _charactermovement) 4))
      (Variables|Dash|SetDashed false))))

(fn ConstructionScript)

(fn TimerPushSetting
  (bind _output_get (Variables|Pushing|SetTimePush (+ (Variables|Pushing|GetTimePush) 0.1)))
  (if (> _output_get (Variables|/Script/RogueBoyard.RogueCharacterStatePushing|GetPushingCoolDown (Variables|Default|GetRogueCharacterStatePushing)))
    (Utilities|Time|ClearandInvalidateTimerbyHandle (Variables|Pushing|GetTimerPushCooldown))
    (Variables|Pushing|SetTimerPushCooldown "")
    (Variables|Pushing|SetTimePush 0.0)))

(fn TimerDashSetting
  (bind _output_get (Variables|Default|SetTimeDash (+ (Variables|Default|GetTimeDash) 0.1)))
  (if (> _output_get (Variables|/Script/RogueBoyard.RogueCharacterStateDash|GetDashCoolDown (Variables|Default|GetRogueCharacterStateDash)))
    (Utilities|Time|ClearandInvalidateTimerbyHandle (Variables|Default|GetTimerDash))
    (Variables|Default|SetTimerDash "")
    (Variables|Default|SetTimeDash 0.0)))

(fn Threshold
  (params (X :type Float%20%28double-precision%29) (Y :type Float%20%28double-precision%29))
  (bind _stickthreshold (Variables|Default|GetStickThreshold))
  (return (and (and (<= X _stickthreshold) (>= X (* _stickthreshold -1.0))) (and (<= Y _stickthreshold) (>= Y (* -1.0 _stickthreshold))))))

(fn TryBuyItem
  (bind _box (Variables|Default|GetBox))
  (bind _overlappingactors (Collision|GetOverlappingActors _box "/Game/RogueBoyard/Props/BP_Shop.BP_Shop_C" :!class /Script/Engine.PrimitiveComponent))
  (if (Utilities|Array|IsNotEmpty _overlappingactors)
    (bind _asbp_shop (Utilities|Casting|CastToBP_Shop (Utilities|Array|Get(acopy) _overlappingactors))
      (:then
        (bind _returnvalue (Class|RogueShop|BuyItem _asbp_shop))
        (Class|RoguePurse|Spend (Variables|Default|GetPurse) (.price _returnvalue))
        (bind _returnvalue_2 (Game|ConstructObjectfromClass (.itemobject _returnvalue)))
        (Utilities|IsValid _returnvalue_2
          (:Is%20Valid
            (Class|RogueItemComponent|SetCurrentItem (Variables|Default|GetUsableItem) _returnvalue_2)
            (return true))
          (:Is%20Not%20Valid
            (Development|PrintString "Bought Item Not Valid" false)
            (return false))))
      (:CastFailed
        (Development|PrintString "NoShop" false)
        (return false)))
    (else
      (Development|PrintString "No Buyable Item in range" false)
      (return false))))

(fn TryPayUrn
  (bind _box (Variables|Default|GetBox))
  (bind _overlappingactors (Collision|GetOverlappingActors _box 0 :!class /Script/Engine.PrimitiveComponent))
  (if (Utilities|Array|IsNotEmpty _overlappingactors)
    (for _array_element _overlappingactors
      (bind _asrogue_auction_urn (Utilities|Casting|CastToRogueAuctionUrn _array_element)
        (:then
          (Class|RogueAuctionUrn|AddBid _asrogue_auction_urn)
          (Class|RoguePurse|Spend (Variables|Default|GetPurse) 1))
        (:CastFailed
          (Development|PrintString "Cast to urn Failed" false)
          (return false))))
    (return true)
    (else
      (Development|PrintString "No urn in Range" false)
      (return false))))

(fn SetForcePush
  (bind _roguecharacterstatepushing (Variables|Default|GetRogueCharacterStatePushing))
  (bind _roguecharacterstatepushing_2 (Variables|Default|GetRogueCharacterStatePushing))
  (Variables|Pushing|SetTimeForce (+ (Variables|Pushing|GetTimeForce) 0.1))
  (if (>= (Variables|Pushing|GetTimeForce) (Variables|/Script/RogueBoyard.RogueCharacterStatePushing|GetTimeMax _roguecharacterstatepushing_2))
    (Variables|Pushing|SetForcePush (Variables|/Script/RogueBoyard.RogueCharacterStatePushing|GetMaxForce _roguecharacterstatepushing_2))
    (Utilities|Time|ClearandInvalidateTimerbyHandle (Variables|Pushing|GetTimerPushing))
    (Variables|Pushing|SetTimerPushing "")
    (CallFunction|FullCharged)
    (else
      (Variables|Pushing|SetForcePush (Math|Float|Lerp (Variables|/Script/RogueBoyard.RogueCharacterStatePushing|GetMinForce _roguecharacterstatepushing) (Variables|/Script/RogueBoyard.RogueCharacterStatePushing|GetMaxForce _roguecharacterstatepushing) (Utilities|InverseLerp (Variables|/Script/RogueBoyard.RogueCharacterStatePushing|GetTimeMin _roguecharacterstatepushing) (Variables|/Script/RogueBoyard.RogueCharacterStatePushing|GetTimeMax _roguecharacterstatepushing) (Variables|Pushing|GetTimeForce)))))))

(fn Paralysis
  (params (ParalysisTime :type Float%20%28double-precision%29))
  (bind _statemachine (Variables|Default|GetStateMachine))
  (if (not (Utilities|Enum|Equal(Enum) (Variables|/Script/RogueBoyard.RogueCharacterStateMachine|GetCurrentStateID _statemachine) "Dead"))
    (Class|RogueCharacterStateMachine|ChangeState _statemachine "Stun")
    (Class|RogueCharacterStateStun|Paralysis (Variables|Default|GetRogueCharacterStateStun) ParalysisTime)))