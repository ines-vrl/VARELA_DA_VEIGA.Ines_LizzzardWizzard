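; BP_Room_Selection maps gamepad input to a room's traps, letting a player select and operate them.
; Left-stick flicks cycle CurrentTrap through the LeftStick array with wraparound, using custom depth on its static mesh to mark the selection.
; The selected trap receives right-stick axes and Interact start/stop, while Push, Power and both Resurect actions start and stop every entry in their own button or trigger arrays.
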(event Input|EnhancedActionEvents|EnhancedInputActionIA_Dash
  (params (ActionValue :type Boolean) (ElapsedSeconds :type Float%20%28double-precision%29) (TriggeredSeconds :type Float%20%28double-precision%29) (InputAction :type Input%20Action%20Object%20Reference :default "/Game/RogueBoyard/Inputs/InputDataPlaytest/IA_Dash.IA_Dash"))
  ;[1 1 1] Right Button
)

(event Input|EnhancedActionEvents|EnhancedInputActionIA_Interact
  (params (ActionValue :type Boolean) (ElapsedSeconds :type Float%20%28double-precision%29) (TriggeredSeconds :type Float%20%28double-precision%29) (InputAction :type Input%20Action%20Object%20Reference :default "/Game/RogueBoyard/Inputs/InputDataPlaytest/IA_Interact.IA_Interact"))
  (bind _currenttrap (Variables|Default|GetCurrentTrap))
  ;[1 1 1] Bottom Button
  (:Started
    (Class|TrapsInput|Started _currenttrap))
  (:Canceled
    (Class|TrapsInput|Stopped _currenttrap :!label _label))
  (:Completed
    (goto _label)))

(event Input|EnhancedActionEvents|EnhancedInputActionIA_Push
  (params (ActionValue :type Boolean) (ElapsedSeconds :type Float%20%28double-precision%29) (TriggeredSeconds :type Float%20%28double-precision%29) (InputAction :type Input%20Action%20Object%20Reference :default "/Game/RogueBoyard/Inputs/InputDataPlaytest/IA_Push.IA_Push"))
  (bind _leftbutton (Variables|Default|GetLeftButton))
  ;[1 1 1] Left Button
  (:Started
    (for _array_element _leftbutton
      (Class|TrapsInput|Started _array_element)))
  (:Canceled
    (for _array_element_2 _leftbutton :!label _label
      (Class|TrapsInput|Stopped _array_element_2)))
  (:Completed
    (goto _label)))

(event Input|EnhancedActionEvents|EnhancedInputActionIA_Resurect_1
  (params (ActionValue :type Boolean) (ElapsedSeconds :type Float%20%28double-precision%29) (TriggeredSeconds :type Float%20%28double-precision%29) (InputAction :type Input%20Action%20Object%20Reference :default "/Game/RogueBoyard/Inputs/InputDataPlaytest/IA_Resurect_1.IA_Resurect_1"))
  (bind _lefttrigger (Variables|Default|GetLeftTrigger))
  ;[1 1 1] Left Trigger
  (:Started
    (for _array_element _lefttrigger
      (Class|TrapsInput|Started _array_element)))
  (:Canceled
    (for _array_element_2 _lefttrigger :!label _label
      (Class|TrapsInput|Stopped _array_element_2)))
  (:Completed
    (goto _label)))

(event Input|EnhancedActionEvents|EnhancedInputActionIA_Resurect_2
  (params (ActionValue :type Boolean) (ElapsedSeconds :type Float%20%28double-precision%29) (TriggeredSeconds :type Float%20%28double-precision%29) (InputAction :type Input%20Action%20Object%20Reference :default "/Game/RogueBoyard/Inputs/InputDataPlaytest/IA_Resurect_2.IA_Resurect_2"))
  (bind _righttrigger (Variables|Default|GetRightTrigger))
  ;[1 1 1] Right Trigger
  (:Started
    (for _array_element _righttrigger
      (Class|TrapsInput|Started _array_element)))
  (:Canceled
    (for _array_element_2 _righttrigger :!label _label
      (Class|TrapsInput|Stopped _array_element_2)))
  (:Completed
    (goto _label)))

(event Input|EnhancedActionEvents|EnhancedInputActionIA_Power
  (params (ActionValue :type Boolean) (ElapsedSeconds :type Float%20%28double-precision%29) (TriggeredSeconds :type Float%20%28double-precision%29) (InputAction :type Input%20Action%20Object%20Reference :default "/Game/RogueBoyard/Inputs/InputDataPlaytest/IA_Power.IA_Power"))
  (bind _topbutton (Variables|Default|GetTopButton))
  ;[1 1 1] Top Button
  (:Started
    (for _array_element _topbutton
      (Class|TrapsInput|Started _array_element)))
  (:Canceled
    (for _array_element_2 _topbutton :!label _label
      (Class|TrapsInput|Stopped _array_element_2)))
  (:Completed
    (goto _label)))

(event Input|EnhancedActionEvents|EnhancedInputActionIA_PTMoves
  (params (ActionValue :type Vector%202D%20Structure) (ElapsedSeconds :type Float%20%28double-precision%29) (TriggeredSeconds :type Float%20%28double-precision%29) (InputAction :type Input%20Action%20Object%20Reference :default "/Game/RogueBoyard/Inputs/InputDataPlaytest/IA_PTMoves.IA_PTMoves"))
  (bind _leftstick (Variables|Default|GetLeftStick))
  (bind _returnvalue (Utilities|Array|Length _leftstick))
  (bind _returnvalue_2 (- _returnvalue 1))
  ;[1 1 1] Left Stick
  (:Started
    (if (> (.x ActionValue) 0.5)
      (Variables|Default|SetValue 1)
      (bind _output_get (Variables|Default|SetLastIndex (+ (Utilities|Array|FindItem _leftstick (Variables|Default|GetCurrentTrap)) (Variables|Default|GetValue)) :!label _label))
      (if (> _output_get _returnvalue_2)
        (Variables|Default|SetLastIndex 0)
        (elif (< _output_get 0)
          (Variables|Default|SetLastIndex _returnvalue_2)))
      (CallFunction|SwitchCustomDepth)
      (elif (< (.x ActionValue) -0.5)
        (Variables|Default|SetValue -1)
        (goto _label)))))

(event Input|EnhancedActionEvents|EnhancedInputActionIA_GamePadMoves
  (params (ActionValue :type Vector%202D%20Structure) (ElapsedSeconds :type Float%20%28double-precision%29) (TriggeredSeconds :type Float%20%28double-precision%29) (InputAction :type Input%20Action%20Object%20Reference :default "/Game/RogueBoyard/Inputs/InputData/IA_GamePadMoves.IA_GamePadMoves"))
  ;[1 1 1] Right Stick
  (:Triggered
    (Class|TrapsInput|Trigger (Variables|Default|GetCurrentTrap) (Math|Vector|MakeVector (.x ActionValue) (.y ActionValue) 0.0) :!label _label))
  (:Completed
    (goto _label)))

(fn ConstructionScript
  (bind _output_get (Variables|Default|SetCurrentTrap (Utilities|Array|Get(acopy) (Variables|Default|GetLeftStick))))
  (Utilities|IsValid (Actor|GetComponentbyClass _output_get "/Script/Engine.StaticMeshComponent")
    (:Is%20Valid
      (Rendering|SetRenderCustomDepth (Actor|GetComponentbyClass _output_get "/Script/Engine.StaticMeshComponent") true))))

(fn SwitchCustomDepth
  (Utilities|IsValid (Actor|GetComponentbyClass (Variables|Default|GetCurrentTrap) "/Script/Engine.StaticMeshComponent")
    (:Is%20Valid
      (Rendering|SetRenderCustomDepth (Actor|GetComponentbyClass (Variables|Default|GetCurrentTrap) "/Script/Engine.StaticMeshComponent") false)
      (bind _output_get (Variables|Default|SetCurrentTrap (Utilities|Array|Get(acopy) (Variables|Default|GetLeftStick) (Variables|Default|GetLastIndex))))
      (Utilities|IsValid (Actor|GetComponentbyClass _output_get "/Script/Engine.StaticMeshComponent")
        (:Is%20Valid
          (Rendering|SetRenderCustomDepth (Actor|GetComponentbyClass _output_get "/Script/Engine.StaticMeshComponent") true))))))