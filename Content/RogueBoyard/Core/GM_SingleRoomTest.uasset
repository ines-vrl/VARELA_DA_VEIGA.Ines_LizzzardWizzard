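; GM_SingleRoomTest is a test game mode that runs a single RogueRoom repeatedly, treating lobby and battle rooms identically.
; Starting finds the room and its pawn, has the master player possess that pawn, sets the room camera, and places other characters as camera follow targets before beginning the room.
; Ending closes the room and resurrects each character, calling StartBattleRoom inside that loop, so the restart runs once per character.
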(event EventStartLobbyRoom
  (bind _returnvalue (Actor|GetActorOfClass "/Script/RogueBoyard.RogueRoom"))
  (bind _output_get (Variables|Default|SetRoom%20Manager _returnvalue))
  (Class|CameraWorldSubsystem|SetCamera (Subsystems|GetCameraWorldSubsystem) (Variables|/Script/RogueBoyard.RogueRoom|GetRoomCamera _output_get))
  (bind _returnvalue_2 (Actor|GetActorOfClass "/Script/RogueBoyard.RogueRoomPawn"))
  (Variables|Default|SetRoom%20Pawn _returnvalue_2)
  (Class|RogueRoom|RoomEnter (Variables|Default|GetRoom%20Manager))
  (Pawn|Possess (Game|GetPlayerController (Variables|Default|GetPlayerMasterIndex)) (Variables|Default|GetRoom%20Pawn))
  (Game|Player|SetViewTargetwithBlend (Game|GetPlayerController 0) (Variables|/Script/RogueBoyard.RogueRoom|GetRoomCamera (Variables|Default|GetRoom%20Manager)) 0.0 "VTBlend_Linear" 0.0 false)
  (for (_array_element _array_index) (Variables|Default|GetCharacters)
    (if (!= _array_index (Variables|Default|GetPlayerMasterIndex))
      (Class|RogueRoom|PlacePlayer (Variables|Default|GetRoom%20Manager) _array_element _array_index)
      (Class|CameraWorldSubsystem|AddFollowTarget (Subsystems|GetCameraWorldSubsystem) _array_element)))
  (Class|RogueRoom|BeginRoom (Variables|Default|GetRoom%20Manager)))

(event EventStartBattleRoom
  (bind _returnvalue (Actor|GetActorOfClass "/Script/RogueBoyard.RogueRoom"))
  (bind _output_get (Variables|Default|SetRoom%20Manager _returnvalue))
  (Class|CameraWorldSubsystem|SetCamera (Subsystems|GetCameraWorldSubsystem) (Variables|/Script/RogueBoyard.RogueRoom|GetRoomCamera _output_get))
  (bind _returnvalue_2 (Actor|GetActorOfClass "/Script/RogueBoyard.RogueRoomPawn"))
  (Variables|Default|SetRoom%20Pawn _returnvalue_2)
  (Class|RogueRoom|RoomEnter (Variables|Default|GetRoom%20Manager))
  (Pawn|Possess (Game|GetPlayerController (Variables|Default|GetPlayerMasterIndex)) (Variables|Default|GetRoom%20Pawn))
  (Game|Player|SetViewTargetwithBlend (Game|GetPlayerController 0) (Variables|/Script/RogueBoyard.RogueRoom|GetRoomCamera (Variables|Default|GetRoom%20Manager)) 0.0 "VTBlend_Linear" 0.0 false)
  (for (_array_element _array_index) (Variables|Default|GetCharacters)
    (if (!= _array_index (Variables|Default|GetPlayerMasterIndex))
      (Class|RogueRoom|PlacePlayer (Variables|Default|GetRoom%20Manager) _array_element _array_index)
      (Class|CameraWorldSubsystem|AddFollowTarget (Subsystems|GetCameraWorldSubsystem) _array_element)))
  (Class|RogueRoom|BeginRoom (Variables|Default|GetRoom%20Manager)))

(event EventEndLobbyRoom
  (Class|RogueRoom|EndRoom (Variables|Default|GetRoom%20Manager))
  (for _array_element (Variables|Default|GetCharacters)
    (Class|RogueCharacter|Resurrect _array_element)
    (Class|RogueGameMode|StartBattleRoom)))

(event EventEndBattleRoom
  (Class|RogueRoom|EndRoom (Variables|Default|GetRoom%20Manager))
  (for _array_element (Variables|Default|GetCharacters)
    (Class|RogueCharacter|Resurrect _array_element)
    (Class|RogueGameMode|StartBattleRoom)))

(fn ConstructionScript)