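; Rogue game mode that runs the room flow, opening a lobby five seconds after play begins and providing start/end events for lobby and battle rooms.
; Each start switches player 0's view to the room camera and places characters, skipping the voted index.
; Lobby end stores the vote; in battle that player controls a RoomPawn (room ID / 2) until the end.
; Both end events advance RogueRoomSubsystem to the next room.
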(event EventBeginPlay
  (Utilities|FlowControl|Delay 5.0)
  (Class|RogueGameMode|StartLobbyRoom))

(event EventEndBattleRoom
  (Class|RogueRoom|EndRoom (Variables|Default|GetActiveRoom))
  (Class|RogueRoomPawn|UnPossesRoom (Utilities|Array|Get(acopy) (Variables|Default|GetRoomPawns) (/ (Variables|/Script/RogueBoyard.RogueRoomSubsystem|GetActiveRoomId (Subsystems|GetRogueRoomSubsystem)) 2)) (Utilities|Array|Get(acopy) (Variables|Default|GetCharacters) (Variables|Default|GetVotedPlayerIndex)))
  (Class|RogueRoom|RoomExit (Variables|Default|GetActiveRoom))
  (Class|RogueRoomSubsystem|NextRoom (Subsystems|GetRogueRoomSubsystem)))

(event EventStartBattleRoom
  (bind _output_get (Variables|Default|SetActiveRoom (Utilities|Array|Get(acopy) (Variables|Default|GetRoomManagers) (Variables|/Script/RogueBoyard.RogueRoomSubsystem|GetActiveRoomId (Subsystems|GetRogueRoomSubsystem)))))
  (Game|Player|SetViewTargetwithBlend (Game|GetPlayerController 0) (Variables|/Script/RogueBoyard.RogueRoom|GetRoomCamera _output_get) 0.0 "VTBlend_Linear" 0.0 false)
  (Class|RogueRoom|RoomEnter (Variables|Default|GetActiveRoom))
  (Class|RogueCharacter|UnPossessCharacter (Utilities|Array|Get(acopy) (Variables|Default|GetCharacters) (Variables|Default|GetVotedPlayerIndex)) (Utilities|Array|Get(acopy) (Variables|Default|GetRoomPawns) (/ (Variables|/Script/RogueBoyard.RogueRoomSubsystem|GetActiveRoomId (Subsystems|GetRogueRoomSubsystem)) 2)))
  (for (_array_element _array_index) (Variables|Default|GetCharacters)
    (if (!= _array_index (Variables|Default|GetVotedPlayerIndex))
      (Class|RogueRoom|PlacePlayer (Variables|Default|GetActiveRoom) _array_element _array_index)))
  (Class|RogueRoom|BeginRoom (Variables|Default|GetActiveRoom)))

(event EventStartLobbyRoom
  (bind _output_get (Variables|Default|SetActiveRoom (Utilities|Array|Get(acopy) (Variables|Default|GetRoomManagers) (Variables|/Script/RogueBoyard.RogueRoomSubsystem|GetActiveRoomId (Subsystems|GetRogueRoomSubsystem)))))
  (Game|Player|SetViewTargetwithBlend (Game|GetPlayerController 0) (Variables|/Script/RogueBoyard.RogueRoom|GetRoomCamera _output_get) 0.0 "VTBlend_Linear" 0.0 false)
  (Class|RogueRoom|RoomEnter (Variables|Default|GetActiveRoom))
  (for (_array_element _array_index) (Variables|Default|GetCharacters)
    (if (!= _array_index (Variables|Default|GetVotedPlayerIndex))
      (Class|RogueRoom|PlacePlayer (Variables|Default|GetActiveRoom) _array_element _array_index)))
  (Class|RogueRoom|BeginRoom (Variables|Default|GetActiveRoom)))

(event EventEndLobbyRoom
  (Class|RogueRoom|EndRoom (Variables|Default|GetActiveRoom))
  (bind _asrogue_lobby_room (Utilities|Casting|CastToRogueLobbyRoom (Variables|Default|GetActiveRoom)))
  (Variables|Default|SetVotedPlayerIndex (Variables|/Script/RogueBoyard.RogueLobbyRoom|GetVotedPlayerIndex _asrogue_lobby_room))
  (Class|RogueRoom|RoomExit (Variables|Default|GetActiveRoom))
  (Class|RogueRoomSubsystem|NextRoom (Subsystems|GetRogueRoomSubsystem)))

(fn ConstructionScript)